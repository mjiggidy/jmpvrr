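; Spring-loaded physical button actor that tagged interactable components push along a configurable, flippable local axis, firing touch and press events.
; Begin overlap records the touch point in actor space; Tick projects the first toucher's displacement onto that axis, moving the mesh up to the actuation distance.
; Full travel triggers a press, rate-limited by a timeout; shorter travel releases it.
; Movement along the facing vector ends the touch, snapping the mesh back.
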(event `self.ReceiveTick`
  (params (DeltaSeconds :type "Float (single-precision)"))
  (bind _returnvalue (`self.GetTransform` self))
  (if (`self.Button Is Touched`)
    (bind _deepest_fella (`self.Get Deepest Interactable`))
    (bind _facing_vector (`self.GetFacingVector` (`self.Push Direction`) (`self.Flip Push Direction`) (`self.btn_placeholder`))) ; Get the desired button direction (WS)
    (bind _returnvalue_2 (`KismetMathLibrary.InverseTransformDirection` _returnvalue _facing_vector))
    (bind _returnvalue_3 (`KismetMathLibrary.ProjectVectorOnToVector` (- (`KismetMathLibrary.InverseTransformLocation` _returnvalue (`SceneComponent.K2_GetComponentLocation` _deepest_fella)) (`self.Initial Touch Location (LS)`)) _returnvalue_2))
    (bind _returnvalue_4 (`KismetMathLibrary.Normal` _returnvalue_3))
    (if (> (`KismetMathLibrary.Dot_VectorVector` _returnvalue_4 (`KismetMathLibrary.Normal` _returnvalue_2)) 0.0)
      (`self.Button Touch End`)
      (else
        (bind _returnvalue_5 (`KismetMathLibrary.FClamp` (`KismetMathLibrary.VSize` _returnvalue_3) 0.0 (`self.Actuation Distance (cm)`)))
        (`SceneComponent.K2_SetRelativeLocation` (`self.btn_placeholder`) (* _returnvalue_4 _returnvalue_5) false false)
        (if (== _returnvalue_5 (`self.Actuation Distance (cm)`))
          (`self.Actuation Reached`)
          (else
            (`self.Actuation Over`)))))))

(event `self.btn_placeholder.OnComponentBeginOverlap`
  (params (OverlappedComponent :type "PrimitiveComponent Object Reference") (OtherActor :type "Actor Object Reference") (OtherComp :type "PrimitiveComponent Object Reference") (OtherBodyIndex :type Integer) (bFromSweep :type Boolean) (SweepResult :type "HitResult Structure (by ref)"))
  (if (and (`KismetSystemLibrary.IsValid` OtherComp) (`ActorComponent.ComponentHasTag` OtherComp (`self.Interactable Tag`)))
    (`KismetArrayLibrary.Array_AddUnique` (`self.Currently Overlapping Components`) OtherComp)
    (if (not (`self.Button Is Touched`))
      (set `self.Initial Touch Location (LS)` (`KismetMathLibrary.InverseTransformLocation` (`self.GetTransform` self) (`SceneComponent.K2_GetComponentLocation` OtherComp)))
      (`self.Button Touch Begin`))))

(event `Actuation Reached`
  (bind _returnvalue (`GameplayStatics.GetTimeSeconds`))
  (if (not (< (- _returnvalue (`self.Time Last Pressed`)) (`self.Timeout Duration (Seconds)`)))
    (set `self.Time Last Pressed` _returnvalue)
    (set `self.Button Is Pressed` true)
    (`self.ButtonPressed`)))

(event `Actuation Over`
  (if (`self.Button Is Pressed`)
    (set `self.Button Is Pressed` false)
    (`self.ButtonUnpressed`)))

(event `Button Touch Begin`
  (set `self.Button Is Touched` true)
  (`self.ButtonTouchStart`))

(event `Button Touch End`
  (set `self.Button Is Touched` false)
  (`KismetArrayLibrary.Array_Clear` (`self.Currently Overlapping Components`))
  (`SceneComponent.ResetRelativeTransform` (`self.btn_placeholder`))
  (`self.ButtonTouchStop`))

(event `Debug`
  (`KismetSystemLibrary.PrintText` (`|FormatText` "Touched? {Is Touched}      Pressed? {Is Pressed}" (`self.Button Is Touched`) (`self.Button Is Pressed`))))

(fn `Get Deepest Interactable`
  (returns (`Deepest Fella` :type "PrimitiveComponent Object Reference"))
  (return (`|GetArrayItem` (`self.Currently Overlapping Components`))))

(fn `Get Interactable Components`
  (params (Components :type "Array of PrimitiveComponent Object Reference"))
  (returns (`Overlapping Interactables` :type "Array of PrimitiveComponent Object Reference"))
  (locals (Interactables :type "Array of PrimitiveComponent Object Reference"))
  (bind _interactables (`local.Interactables`))
  (for _array_element Components
    (if (`ActorComponent.ComponentHasTag` _array_element (`self.Interactable Tag`))
      (`KismetArrayLibrary.Array_Add` _interactables _array_element)))
  (return _interactables))

(fn `GetFacingVector`
  (params (Direction :type "/Game/Caldoria/Blueprints/Enums/E_VectorDirections Enum" :default "NewEnumerator0") (Flip :type Boolean) (Component :type "SceneComponent Object Reference"))
  (returns (`Facing Vector` :type "Vector Structure"))
  (locals (Multiplier :type "Float (double-precision)" :default 1.0) (ChosenVector :type "Vector Structure"))
  (if Flip
    (set `local.Multiplier` -1.0))
  (switch `/Game/Caldoria/Blueprints/Enums/E_VectorDirections` Direction
    (:`NewEnumerator0`
      (set `local.ChosenVector` (`SceneComponent.GetForwardVector` Component)))
    (:`NewEnumerator1`
      (set `local.ChosenVector` (`SceneComponent.GetRightVector` Component)))
    (:`NewEnumerator2`
      (set `local.ChosenVector` (`SceneComponent.GetUpVector` Component))))
  (return (* (`local.ChosenVector`) (`local.Multiplier`))))

(fn `UserConstructionScript`
  (locals (NewLocalVar :type "BoxSphereBounds Structure"))
  (bind _btn_placeholder (`self.btn_placeholder`))
  (bind _returnvalue (`SceneComponent.K2_GetComponentLocation` _btn_placeholder))
  (`|ExecutionSequence`
    (:`then_0`
      ;[1 1 1] Static Mesh Setup
      (`StaticMeshComponent.SetStaticMesh` (`self.btn_placeholder`) (`self.Button Static Mesh`)))
    (:`then_1`
      ;[1 1 1] Display Facing Vector
      (bind _facing_vector (`self.GetFacingVector` (`self.Push Direction`) (`self.Flip Push Direction`) _btn_placeholder))
      (`KismetSystemLibrary.DrawDebugArrow` (+ _facing_vector _returnvalue) _returnvalue 10.0 (struct :`R` 1.0 :`A` 1.0) 10.0))
    (:`then_2`)))