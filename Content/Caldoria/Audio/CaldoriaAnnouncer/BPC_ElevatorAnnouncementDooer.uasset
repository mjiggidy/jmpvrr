(event `Announce Floor`
  (params (Floor :type "/Game/Caldoria/Blueprints/BP_Elevator_Hallway Object Reference"))
  (bind _speaker (`self.Speaker`))
  (bind _object (`|LoadAsset` (`/Game/Caldoria/Blueprints/BP_Elevator_Hallway.Floor Announcement` Floor))
    (:`Completed`
      (bind _assound_wave (cast `SoundWave` _object))
      (`AudioComponent.SetSound` _speaker _assound_wave)
      (`AudioComponent.Play` _speaker 0.0))))

(fn `Set Speaker`
  (params (Speaker :type "AudioComponent Object Reference"))
  (set `self.Speaker` Speaker))