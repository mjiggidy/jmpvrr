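; Controller that turns tagged walls and doors into environment projection surfaces, starting on player overlap and switching to a random environment on later overlaps.
; Tagged meshes get cached dynamic instances of a template material with copied overrides, mapped to originals for restoring.
; Environment changes async-load a cubemap while a timeline fades material brightness, power, pixelation and wall color.
; Begin dims the overhead rect light; End fades back and restores original materials.
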(event `Environment Fade`
  (params (`To Map Brightness` :type "Float (double-precision)") (`To Map Power` :type "Float (double-precision)") (`To Pixel Density` :type "Float (double-precision)") (`To Wall Color` :type "LinearColor Structure"))
  (bind (_wall_base_color _map_power _map_brightness _pixel_power) (`self.Get Current Material Properties`))
  (bind (_direction _fader) (`Timeline|Timeline` :!via `PlayFromStart`)
    (:`Update`
      (`self.Set Projection Material Properties` (`KismetMathLibrary.Lerp` _map_brightness `To Map Brightness` _fader) (`KismetMathLibrary.Lerp` _map_power `To Map Power` _fader) (`KismetMathLibrary.Lerp` _pixel_power `To Pixel Density` _fader) (`KismetMathLibrary.LinearColorLerp` _wall_base_color `To Wall Color` _fader)))))

(event `Set Environment Map`
  (params (Environment :type "/Game/Caldoria/Blueprints/_TEMP_ENVIRON/PDA_Environ_Environment Object Reference"))
  (bind _object (`|LoadAsset` (`/Game/Caldoria/Blueprints/_TEMP_ENVIRON/PDA_Environ_Environment.Cubemap` Environment))
    (:`then`
      (`self.Environment Fade` 0.0 1.0 1.0 (`self.!Base Wall Color Default`)))
    (:`Completed`
      (`KismetSystemLibrary.Delay` 1.1) ; ugh no
      (bind _astexture_cube (cast `TextureCube` _object))
      (bind _values (`BlueprintMapLibrary.Map_Values` (`self.Dynamic Materials`)))
      (for _array_element _values
        (`MaterialInstanceDynamic.SetTextureParameterValue` _array_element (`self.Material Cubemap Param`) _astexture_cube))
      (`self.Environment Fade` (`/Game/Caldoria/Blueprints/_TEMP_ENVIRON/PDA_Environ_Environment.Map Brightness` Environment) (`/Game/Caldoria/Blueprints/_TEMP_ENVIRON/PDA_Environ_Environment.Map Power` Environment) (`/Game/Caldoria/Blueprints/_TEMP_ENVIRON/PDA_Environ_Environment.Pixel Power` Environment) (`self.Base Wall Color Faded`)))))

(event `Random Environment`
  (`self.Set Environment Map` (`KismetArrayLibrary.Array_Random` (`self.Environments`))))

(event `self.ReceiveBeginPlay`)

(event `Begin Eviron`
  (`self.Setup Projection`)
  (set `self.Overhead Default Intensity` (`LightComponentBase.Intensity` (`RectLight.RectLightComponent` (`self.Overhead Light`))))
  (`self.Fade Light` (`self.Overhead Faded Intensity`))
  (set `self.Environ Active` true))

(event `End Environ`
  (if (`self.Environ Active`)
    (`self.Environment Fade` 0.0 1.0 1.0 (`self.!Base Wall Color Default`))
    (`KismetSystemLibrary.Delay` 0.75)
    (`self.Fade Light` (`self.Overhead Default Intensity`))
    (`KismetSystemLibrary.Delay` 1.0)
    (`self.Unset Materials`)
    (set `self.Environ Active` false)))

(event `Setup Projection`
  (bind _environ_static_meshes (`self.Load Surfaces`))
  (bind _output_get (set `self.Projection Surfaces` _environ_static_meshes))
  (for _array_element _output_get
    (bind _projection_material (`self.Get Projection Material From Static Material` (`PrimitiveComponent.GetMaterial` _array_element 0)))
    (`PrimitiveComponent.SetMaterial` _array_element 0 _projection_material))
  (`self.Random Environment`))

(event `Unset Materials`
  (bind _projection_surfaces (`self.Projection Surfaces`))
  (for _array_element _projection_surfaces
    (bind _asmaterial_instance_dynamic (cast `MaterialInstanceDynamic` (`PrimitiveComponent.GetMaterial` _array_element 0)))
    (bind _static_material (`self.Get Static Material From Projection Material` _asmaterial_instance_dynamic))
    (`PrimitiveComponent.SetMaterial` _array_element 0 _static_material))
  (`KismetArrayLibrary.Array_Clear` _projection_surfaces))

(event `Fade Light`
  (params (`To Intensity` :type "Float (double-precision)"))
  (bind _output_get (set `self.Overhead Current Intensity` (`LightComponentBase.Intensity` (`RectLight.RectLightComponent` (`self.Overhead Light`)))))
  (bind (_direction _newtrack_0) (`Timeline|Timeline_0` :!via `PlayFromStart`)
    (:`Update`
      (`LightComponent.SetIntensity` (`RectLight.RectLightComponent` (`self.Overhead Light`)) (`KismetMathLibrary.Lerp` _output_get `To Intensity` _newtrack_0)))))

(event `self.Temp Box.OnComponentBeginOverlap`
  (params (OverlappedComponent :type "PrimitiveComponent Object Reference") (OtherActor :type "Actor Object Reference") (OtherComp :type "PrimitiveComponent Object Reference") (OtherBodyIndex :type Integer) (bFromSweep :type Boolean) (SweepResult :type "HitResult Structure (by ref)"))
  (if (== OtherActor (`GameplayStatics.GetPlayerPawn` 0))
    (if (`self.Environ Active`)
      (`self.Random Environment`)
      (else
        (`self.Begin Eviron`)))))

(fn `Get Current Material Properties`
  (returns (`Wall Base Color` :type "LinearColor Structure") (`Map Power` :type "Float (double-precision)") (`Map Brightness` :type "Float (double-precision)") (`Pixel Power` :type "Float (double-precision)"))
  (bind _values (`BlueprintMapLibrary.Map_Values` (`self.Dynamic Materials`)))
  (bind _output (`|GetArrayItem` _values))
  (bind _returnvalue (`MaterialInstanceDynamic.K2_GetScalarParameterValue` _output (`self.Material Emission Brightness`)))
  (bind _returnvalue_2 (`MaterialInstanceDynamic.K2_GetScalarParameterValue` _output (`self.Material Emission Power`)))
  (bind _returnvalue_3 (`MaterialInstanceDynamic.K2_GetScalarParameterValue` _output (`self.Material Pixel Power`)))
  (bind _returnvalue_4 (`MaterialInstanceDynamic.K2_GetVectorParameterValue` _output (`self.Material Wall Albedo Param`)))
  (return _returnvalue_4 _returnvalue_2 _returnvalue _returnvalue_3))

(fn `Get Material From Actor`
  (params (Actor :type "Actor Object Reference"))
  (returns (`Material Instance` :type "MaterialInterface Object Reference"))
  (bind _asstatic_mesh_actor (cast `StaticMeshActor` Actor))
  (return (`|GetArrayItem` (`MeshComponent.GetMaterials` (`StaticMeshActor.StaticMeshComponent` _asstatic_mesh_actor)))))

(fn `Get Projection Material From Static Material`
  (params (`Material Interface` :type "MaterialInterface Object Reference"))
  (returns (`Projection Material` :type "MaterialInstanceDynamic Object Reference"))
  (bind _dynamic_materials (`self.Dynamic Materials`))
  (bind (_value _returnvalue) (`BlueprintMapLibrary.Map_Find` _dynamic_materials `Material Interface`))
  (if _returnvalue
    (return _value)
    (else
      ;[1 1 1] Almost Works -- But Static Switch Parameters (Art Flip) Don't Copy
      (bind _asmaterial_instance (cast `MaterialInstance` `Material Interface`))
      (bind _returnvalue_2 (`KismetSystemLibrary.LoadAsset_Blocking` (`self.Environ Material Template`)))
      (bind _asmaterial_interface (cast `MaterialInterface` _returnvalue_2))
      (bind _returnvalue_3 (`KismetMaterialLibrary.CreateDynamicMaterialInstance` _asmaterial_interface))
      (`MaterialInstanceDynamic.CopyParameterOverrides` _returnvalue_3 _asmaterial_instance)
      (`BlueprintMapLibrary.Map_Add` _dynamic_materials `Material Interface` _returnvalue_3)
      (return _returnvalue_3))))

(fn `Get Static Material From Projection Material`
  (params (`Projection Material` :type "MaterialInstanceDynamic Object Reference"))
  (returns (`Static Material` :type "MaterialInterface Object Reference"))
  (bind _dynamic_materials (`self.Dynamic Materials`))
  (bind _keys (`BlueprintMapLibrary.Map_Keys` _dynamic_materials))
  (for _array_element _keys
    (if (== `Projection Material` (`BlueprintMapLibrary.Map_Find` _dynamic_materials _array_element))
      (return _array_element))))

(fn `Load Surfaces`
  (returns (`Environ Static Meshes` :type "Array of StaticMeshComponent Object Reference"))
  (locals (`Static Mesh Components` :type "Array of StaticMeshComponent Object Reference"))
  (bind _static_mesh_components (`local.Static Mesh Components`))
  (bind _outactors (`GameplayStatics.GetAllActorsWithTag` "Environ"))
  (for _array_element _outactors
    (bind _asstatic_mesh_actor (cast `StaticMeshActor` _array_element)
      (:`then`
        (`KismetArrayLibrary.Array_AddUnique` _static_mesh_components (`StaticMeshActor.StaticMeshComponent` _asstatic_mesh_actor)))
      (:`CastFailed`
        (bind _asbp_door_apartment (cast `/Game/Caldoria/Blueprints/BP_Door_Apartment` _array_element)
          (:`then`
            (`KismetArrayLibrary.Array_Append` _static_mesh_components (`self.GetComponentsByTag` _asbp_door_apartment "/Script/Engine.StaticMeshComponent" "Environ")))
          (:`CastFailed`
            (bind _asbp_door_hallway (cast `/Game/Caldoria/Blueprints/BP_Door_Hallway` _array_element))
            (`KismetArrayLibrary.Array_Append` _static_mesh_components (`self.GetComponentsByTag` _asbp_door_hallway "/Script/Engine.StaticMeshComponent" "Environ")))))))
  (return _static_mesh_components))

(fn `Set Projection Material Properties`
  (params (`Map Brightness` :type "Float (double-precision)") (`Map Power` :type "Float (double-precision)") (`Pixel Power` :type "Float (double-precision)") (`Wall Color` :type "LinearColor Structure"))
  (bind _values (`BlueprintMapLibrary.Map_Values` (`self.Dynamic Materials`)))
  (for _array_element _values
    (`MaterialInstanceDynamic.SetScalarParameterValue` _array_element (`self.Material Emission Brightness`) `Map Brightness`)
    (`MaterialInstanceDynamic.SetScalarParameterValue` _array_element (`self.Material Emission Power`) `Map Power`)
    (`MaterialInstanceDynamic.SetScalarParameterValue` _array_element (`self.Material Pixel Power`) `Pixel Power`)
    (`MaterialInstanceDynamic.SetVectorParameterValue` _array_element (`self.Material Wall Albedo Param`) `Wall Color`)))

(fn `UserConstructionScript`)