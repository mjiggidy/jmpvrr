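; Elevator keypad that relays floor requests from its buttons and reflects the elevator's queue and arrivals on them.
; Buttons are spawned as child BP_Elevator_Keypad_Button actors in a column-wrapped grid, though SetupButtons here adds only one.
; Requests pass through a timer-based lockout before being broadcast, limiting repeated presses.
; Queue and arrival events look up the matching button by floor and switch it on or off.
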(event `self.ReceiveBeginPlay`
  (`self.Setup Buttons`))

(event `Keypad Requested Floor`
  (params (`Requested Floor` :type "/Game/Caldoria/Blueprints/BP_Elevator_Hallway Object Reference"))
  (if (not (`self.Timeout Active`))
    (`self.Start Timeout`)
    (`self.FloorRequested` `Requested Floor`)))

(event `Floor Added To Queue`
  (params (`Queued Floor` :type "/Game/Caldoria/Blueprints/BP_Elevator_Hallway Object Reference"))
  (bind _keypad_button (`self.GetButtonForFloor` `Queued Floor`))
  (`/Game/Caldoria/Blueprints/BP_Elevator_Keypad_Button.TurnButtonOn` _keypad_button false))

(event `Floor Removed From Queue`
  (params (`Removed Floor` :type "/Game/Caldoria/Blueprints/BP_Elevator_Hallway Object Reference"))
  (bind _keypad_button (`self.GetButtonForFloor` `Removed Floor`))
  (`/Game/Caldoria/Blueprints/BP_Elevator_Keypad_Button.TurnButtonOff` _keypad_button))

(event `Arrived At Floor`
  (params (`At Floor` :type "/Game/Caldoria/Blueprints/BP_Elevator_Hallway Object Reference"))
  (bind _keypad_button (`self.GetButtonForFloor` `At Floor`))
  (`/Game/Caldoria/Blueprints/BP_Elevator_Keypad_Button.TurnButtonOn` _keypad_button true))

(event `Start Timeout`
  (set `self.Timeout Active` true)
  (`KismetSystemLibrary.K2_SetTimerDelegate` (`|CreateDelegate` :!event `End Timeout`) (`self.Timeout Duration (s)`)))

(event `End Timeout`
  (set `self.Timeout Active` false))

(fn `Add Floor Button`
  (params (`New Floor` :type "/Game/Caldoria/Blueprints/BP_Elevator_Hallway Object Reference") (`Key Mode` :type "/Game/Caldoria/Blueprints/Enums/E_Elevator_Keypad_Button_Modes Enum" :default "NewEnumerator0"))
  (returns (`New Button` :type "/Game/Caldoria/Blueprints/BP_Elevator_Keypad_Button Object Reference"))
  (bind _returnvalue (`KismetArrayLibrary.Array_Length` (`self.Keys`)))
  (bind _returnvalue_2 (`AddComponent|NODE_AddChildActorComponent-0` :`RelativeTransform` (`KismetMathLibrary.MakeTransform` (`KismetMathLibrary.MakeVector` 0.0 (* (* (mod _returnvalue (`self.Columns`)) (`self.Key Spacing`)) -1.0) (* (* (`KismetMathLibrary.FFloor` (/ _returnvalue (`self.Columns`))) (`self.Key Spacing`)) -1.0)))))
  (bind _asbp_elevator_keypad_button (cast `/Game/Caldoria/Blueprints/BP_Elevator_Keypad_Button` (`ChildActorComponent.ChildActor` _returnvalue_2)))
  (`/Game/Caldoria/Blueprints/BP_Elevator_Keypad_Button.SetupButton` _asbp_elevator_keypad_button `Key Mode` `New Floor`)
  (`KismetArrayLibrary.Array_Add` (`self.Keys`) _asbp_elevator_keypad_button)
  (add `/Game/Caldoria/Blueprints/BP_Elevator_Keypad_Button.FloorRequested` _asbp_elevator_keypad_button (`|CreateDelegate` :!event `Keypad Requested Floor`))
  (return _asbp_elevator_keypad_button))

(fn `GetButtonForFloor`
  (params (Floor :type "/Game/Caldoria/Blueprints/BP_Elevator_Hallway Object Reference"))
  (returns (`Keypad Button` :type "/Game/Caldoria/Blueprints/BP_Elevator_Keypad_Button Object Reference"))
  (for _array_element (`self.Keys`)
    (if (== (`/Game/Caldoria/Blueprints/BP_Elevator_Keypad_Button.Floor` _array_element) Floor)
      (return _array_element))))

(fn `SetButtonNumber`
  (params (`Floor Number` :type String) (`Static Mesh Instance` :type "StaticMeshComponent Object Reference"))
  (bind _asmaterial_instance_dynamic (cast `MaterialInstanceDynamic` (`PrimitiveComponent.GetMaterial` `Static Mesh Instance` 0)))
  (`MaterialInstanceDynamic.SetScalarParameterValue` _asmaterial_instance_dynamic "Floor Number" (`KismetStringLibrary.Conv_StringToDouble` `Floor Number`)))

(fn `Setup Buttons`
  (`self.Add Floor Button` null "NewEnumerator1"))

(fn `UserConstructionScript`)