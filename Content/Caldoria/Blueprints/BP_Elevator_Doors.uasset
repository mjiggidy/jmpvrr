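; Caldoria elevator hallway doors, two panels that slide open and closed at a caller-set play rate.
; The construction script caches closed positions and derives open ones, with both panels sliding toward -X.
; OpenDoors and CloseDoors run separate timelines lerping from the current positions, so reversing mid-motion is smooth.
; DoorStateChanged fires when opening starts but only once closing finishes; helpers expose open/locked state and map floor numbers to indices.
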(event `self.ReceiveBeginPlay`)

(event `Test Open Doors`
  (`self.Open Doors` 1.0))

(event `Test Close Doors`
  (`self.Close Doors` 1.0))

(event `Open Doors`
  (params (`Open Rate` :type "Float (double-precision)" :default 1.0))
  (if (not (`self.DoorIsOpen`))
    (set `self.DoorIsOpen` true)
    (`self.DoorStateChanged` true)
    (`TimelineComponent.Stop` (`self.Doors Closing`))
    (set `self.Door L Current` (`SceneComponent.RelativeLocation` (`self.Cal_Elevator_Hallway_Door_L`)))
    (set `self.Door R Current` (`SceneComponent.RelativeLocation` (`self.Cal_Elevator_Hallway_Door_R`)))
    (`TimelineComponent.SetPlayRate` (`self.Doors Opening`) `Open Rate`)
    (bind (_direction _door_offset) (`Timeline|Doors Opening` :!via `PlayFromStart`)
      (:`Update`
        (`SceneComponent.K2_SetRelativeLocation` (`self.Cal_Elevator_Hallway_Door_L`) (`KismetMathLibrary.VLerp` (`self.Door L Current`) (`self.Door L Destination`) _door_offset) false false)
        (`SceneComponent.K2_SetRelativeLocation` (`self.Cal_Elevator_Hallway_Door_R`) (`KismetMathLibrary.VLerp` (`self.Door R Current`) (`self.Door R Destination`) _door_offset) false false)))))

(event `Close Doors`
  (params (`Close Rate` :type "Float (double-precision)" :default 1.0))
  (if (`self.DoorIsOpen`)
    (set `self.DoorIsOpen` false)
    (`TimelineComponent.Stop` (`self.Doors Opening`))
    (set `self.Door L Current` (`SceneComponent.RelativeLocation` (`self.Cal_Elevator_Hallway_Door_L`)))
    (set `self.Door R Current` (`SceneComponent.RelativeLocation` (`self.Cal_Elevator_Hallway_Door_R`)))
    (`TimelineComponent.SetPlayRate` (`self.Doors Closing`) `Close Rate`)
    (bind (_direction _door_offset) (`Timeline|Doors Closing` :!via `PlayFromStart`)
      (:`Update`
        (`SceneComponent.K2_SetRelativeLocation` (`self.Cal_Elevator_Hallway_Door_L`) (`KismetMathLibrary.VLerp` (`self.Door L Current`) (`self.Door L Initial`) _door_offset) false false)
        (`SceneComponent.K2_SetRelativeLocation` (`self.Cal_Elevator_Hallway_Door_R`) (`KismetMathLibrary.VLerp` (`self.Door R Current`) (`self.Door R Initial`) _door_offset) false false))
      (:`Finished`
        (`self.DoorStateChanged` false)))))

(fn `FloorIndexFromNumber`
  (params (`Floor Number` :type String))
  (returns (`Floor Index` :type "Float (double-precision)"))
  (locals (`Special Lookup` :type "Map of String to Float (double-precision)") (Unknown :type "Float (double-precision)" :default 6.0))
  (bind (_value _returnvalue) (`BlueprintMapLibrary.Map_Find` (`local.Special Lookup`) `Floor Number`))
  (if (`KismetStringLibrary.IsNumeric` `Floor Number`)
    (if (< `Floor Number` (`local.Unknown`))
      (return (`KismetStringLibrary.Conv_StringToDouble` `Floor Number`))
      (else
        _))
    (elif _returnvalue
      (return _value)
      (else
        _)))
  (return (`local.Unknown`)))

(fn `Get Door Offset`
  (params (`Door Initial` :type "Vector Structure") (`Open Amount` :type "Float (double-precision)") (`Open Direction` :type "/Game/Caldoria/Blueprints/E_OpenDirection Enum" :default "NewEnumerator0"))
  (returns (`Door Destination` :type "Vector Structure"))
  (locals (Door :type "Transform Structure"))
  (switch `/Game/Caldoria/Blueprints/E_OpenDirection` `Open Direction`
    (:`NewEnumerator0`
      (return (`KismetMathLibrary.MakeVector` (- `Door Initial_X` `Open Amount`) `Door Initial_Y` `Door Initial_Z`)))
    (:`NewEnumerator1`
      (return (`KismetMathLibrary.MakeVector` (+ `Door Initial_X` `Open Amount`) `Door Initial_Y` `Door Initial_Z`)))))

(fn `GetIsLocked`
  (returns (IsLocked :type Boolean))
  (return (`self.DoorIsLocked`)))

(fn `GetIsOpen`
  (returns (`Door Is Open` :type Boolean))
  (return (`self.DoorIsOpen`)))

(fn `UserConstructionScript`
  (`|ExecutionSequence`
    (:`then_3`
      ;[1 1 1] Initial Closed Door State
      (bind _output_get (set `self.Door L Initial` (`SceneComponent.RelativeLocation` (`self.Cal_Elevator_Hallway_Door_L`))))
      (bind _output_get_2 (set `self.Door R Initial` (`SceneComponent.RelativeLocation` (`self.Cal_Elevator_Hallway_Door_R`))))
      (bind _output_get_3 (set `self.Door L Destination` (`KismetMathLibrary.MakeVector` (- (.x _output_get) 74.0) (.y _output_get) (.z _output_get))))
      (set `self.Door R Destination` (`KismetMathLibrary.MakeVector` (- (.x _output_get_3) 75.0) (.y _output_get_2) (.z _output_get_2))))))