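; Caldoria kiosk actor that animates between a ready and a retracted state through Prepare and Retract events.
; Prepare chains timelines to fade in the light rail and rect light, pitch the screen, then slide the projector cartridge to center while its gears turn with the offset.
; Retract turns the light off, fades the rail and pivots the screen back, leaving the cartridge in place.
; The construction script creates the rail's dynamic material, sets timeline rates and poses screen and cartridge.
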(event `Prepare`
  (bind _temp_cal_kiosk_screen (`self.temp_cal_kiosk_screen`))
  (bind (_relativerotation_roll _relativerotation_pitch) (`KismetMathLibrary.BreakRotator` (`SceneComponent.RelativeRotation` _temp_cal_kiosk_screen)))
  (bind (_direction _newtrack_0) (`Timeline|TL Light Fade On` :!via `PlayFromStart`)
    (:`Update`
      (`self.Set Light Rail Glow` _newtrack_0))
    (:`Finished`
      (`SceneComponent.SetVisibility` (`self.RectLight`) true false)
      (`KismetSystemLibrary.Delay` (`self.Board Roate Delay`))
      (bind _output_get (set `self.Initial Relative Rotation Y (Pitch)` _relativerotation_pitch))
      (bind (_direction_2 _newtrack_1) (`Timeline|TL Board Pivot Down` :!via `PlayFromStart`)
        (:`Update`
          (`SceneComponent.K2_SetRelativeRotation` _temp_cal_kiosk_screen (`KismetMathLibrary.MakeRotator` 0.0 (`KismetMathLibrary.Lerp` _output_get (`self.End Rotation`) _newtrack_1)) false false))
        (:`Finished`
          (`KismetSystemLibrary.Delay` 1.0)
          (bind (_direction_3 _newtrack_0_2) (`Timeline|Projector Ready` :!via `PlayFromStart`)
            (:`Update`
              (`self.SetCartridgePositionOffset` (`KismetMathLibrary.Lerp` (`self.Projector Rest Position`) (`self.Projector Center Position`) _newtrack_0_2)))))))))

(event `Retract`
  (bind _temp_cal_kiosk_screen (`self.temp_cal_kiosk_screen`))
  (bind (_relativerotation_roll _relativerotation_pitch) (`KismetMathLibrary.BreakRotator` (`SceneComponent.RelativeRotation` _temp_cal_kiosk_screen)))
  (`SceneComponent.SetVisibility` (`self.RectLight`) false false)
  (bind (_direction _newtrack_0) (`Timeline|TL Light Fade Off` :!via `PlayFromStart`)
    (:`Update`
      (`self.Set Light Rail Glow` _newtrack_0)
      (`KismetSystemLibrary.Delay` (`self.Board Roate Delay`))
      (bind _output_get (set `self.Initial Relative Rotation Y (Pitch)` _relativerotation_pitch))
      (bind (_direction_2 _newtrack_1) (`Timeline|TL Board Pivot Return` :!via `PlayFromStart`)
        (:`Update`
          (`SceneComponent.K2_SetRelativeRotation` _temp_cal_kiosk_screen (`KismetMathLibrary.MakeRotator` 0.0 (`KismetMathLibrary.Lerp` _output_get (`self.Initial Rotation`) _newtrack_1)) false false))))))

(fn `Set Light Rail Glow`
  (params (`Glow Amount` :type "Float (double-precision)"))
  (`MaterialInstanceDynamic.SetScalarParameterValue` (`self.Light Rail Dynamic Material`) "Light Fade" `Glow Amount`))

(fn `SetCartridgePositionOffset`
  (params (Offset :type "Float (double-precision)"))
  (`SceneComponent.K2_SetRelativeLocation` (`self.temp_cal_kiosk_cartridge`) (+ (`self.Projector Initial Position`) (`KismetMathLibrary.MakeVector` 0.0 Offset)) false false)
  (`SceneComponent.K2_SetRelativeRotation` (`self.temp_cal_kiosk_cartridge_gears`) (`KismetMathLibrary.NormalizedDeltaRotator` (`self.Gear Initial Rotation`) (`KismetMathLibrary.MakeRotator` (* Offset (`self.Gear Rotation Speed`)))) false false))

(fn `UserConstructionScript`
  (bind _returnvalue (/ 1.0 (`self.Rate`)))
  (bind _returnvalue_2 (/ 1.0 (`self.Light Fade Speed`)))
  (`|ExecutionSequence`
    (:`then_0`
      (bind _returnvalue_3 (`PrimitiveComponent.CreateDynamicMaterialInstance` (`self.temp_cal_kiosk_rails`) 0 null "None"))
      (bind _output_get (set `self.Light Rail Dynamic Material` _returnvalue_3))
      (`MaterialInstanceDynamic.SetScalarParameterValue` _output_get "Light Intensity" (`self.Max Light Intensity`))
      (`self.Set Light Rail Glow` 0.0))
    (:`then_1`
      (`TimelineComponent.SetPlayRate` (`self.TL Board Pivot Down`) _returnvalue)
      (`TimelineComponent.SetPlayRate` (`self.TL Board Pivot Return`) _returnvalue)
      (`TimelineComponent.SetPlayRate` (`self.TL Light Fade On`) _returnvalue_2)
      (`TimelineComponent.SetPlayRate` (`self.TL Light Fade Off`) _returnvalue_2))
    (:`then_2`
      (`SceneComponent.K2_SetRelativeRotation` (`self.temp_cal_kiosk_screen`) (`KismetMathLibrary.MakeRotator` 0.0 (`self.Initial Rotation`)) false false))
    (:`then_3`
      (set `self.Projector Initial Position` (`SceneComponent.RelativeLocation` (`self.temp_cal_kiosk_cartridge`)))
      (set `self.Gear Initial Rotation` (`SceneComponent.RelativeRotation` (`self.temp_cal_kiosk_cartridge_gears`))))
    (:`then_4`
      (if (`self.Start Activated`)
        (`self.SetCartridgePositionOffset` (`self.Projector Center Position`))
        (else
          (`self.SetCartridgePositionOffset` (`self.Projector Rest Position`)))))))