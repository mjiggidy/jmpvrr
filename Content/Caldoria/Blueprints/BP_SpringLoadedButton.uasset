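; BP_SpringLoadedButton is a button actor that detects when components tagged "Interact" touch it and signals touch start and stop.
; Its construction script assigns the mesh and fits a padded, offset collision box to the mesh bounds.
; Overlaps fire ButtonTouchStart on first contact and ButtonTouchStop once no tagged components remain.
; A stop handler is bound during construction, and a reset event restores the mesh's relative transform.
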(event `self.ReceiveBeginPlay`)

(event `self.Collision Bounds.OnComponentBeginOverlap`
  (params (OverlappedComponent :type "PrimitiveComponent Object Reference") (OtherActor :type "Actor Object Reference") (OtherComp :type "PrimitiveComponent Object Reference") (OtherBodyIndex :type Integer) (bFromSweep :type Boolean) (SweepResult :type "HitResult Structure (by ref)"))
  (`KismetSystemLibrary.PrintString` "Uh")
  (if (and (`KismetSystemLibrary.IsValid` OtherComp) (`ActorComponent.ComponentHasTag` OtherComp "Interact"))
    (`KismetArrayLibrary.Array_AddUnique` (`self.Currently Overlapping Components`) OtherComp)
    (if (not (`self.Button Being Touched`))
      (set `self.Button Being Touched` true)
      (`self.ButtonTouchStart`)
      (`KismetSystemLibrary.PrintString` "Start"))))

(event `self.Collision Bounds.OnComponentEndOverlap`
  (params (OverlappedComponent :type "PrimitiveComponent Object Reference") (OtherActor :type "Actor Object Reference") (OtherComp :type "PrimitiveComponent Object Reference") (OtherBodyIndex :type Integer))
  (if (`ActorComponent.ComponentHasTag` OtherComp "Interact")
    (bind _overlapping_interactables (`self.Has Interactable Components` (`PrimitiveComponent.GetOverlappingComponents` (`self.Collision Bounds`))))
    (if (not (`KismetMathLibrary.Conv_IntToBool` (`KismetArrayLibrary.Array_Length` _overlapping_interactables)))
      (`KismetArrayLibrary.Array_RemoveItem` (`self.Currently Overlapping Components`) OtherComp)
      (set `self.Button Being Touched` false)
      (`self.ButtonTouchStop`))))

(event `Reset Button Situation`
  (`SceneComponent.ResetRelativeTransform` (`self.Button Mesh`))
  (`KismetSystemLibrary.PrintString` "Done"))

(fn `Has Interactable Components`
  (params (Components :type "Array of PrimitiveComponent Object Reference"))
  (returns (`Overlapping Interactables` :type "Array of PrimitiveComponent Object Reference"))
  (locals (Interactables :type "Array of PrimitiveComponent Object Reference"))
  (bind _interactables (`local.Interactables`))
  (for _array_element Components
    (if (`ActorComponent.ComponentHasTag` _array_element "Interact")
      (`KismetArrayLibrary.Array_Add` _interactables _array_element)))
  (return _interactables))

(fn `UserConstructionScript`
  (bind _collision_bounds (`self.Collision Bounds`))
  (bind (_origin _boxextent) (`KismetSystemLibrary.GetComponentBounds` (`self.Button Mesh`)))
  (bind _returnvalue (+ _boxextent (`self.Bounds Padding`)))
  (`|ExecutionSequence`
    (:`then_0`
      ;[1 1 1] Static Mesh Setup
      (`StaticMeshComponent.SetStaticMesh` (`self.Button Mesh`) (`self.Button Static Mesh`)))
    (:`then_1`
      ;[1 1 1] Collision Setup
      (`KismetSystemLibrary.PrintString` (`KismetTextLibrary.Conv_TextToString` (`|FormatText` "Hey I saw {this}" (`KismetStringLibrary.Conv_VectorToString` _returnvalue))))
      (`SceneComponent.K2_SetWorldLocation` _collision_bounds (+ (`self.Bounds Position Offset`) _origin) false false)
      (`BoxComponent.SetBoxExtent` _collision_bounds _returnvalue true))
    (:`then_2`
      ;[1 1 1] Bind Events
      (add `self.ButtonTouchStop` (`|CreateDelegate` :!event `Reset Button Situation`)))))