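; Caldoria apartment door that toggles open when an "Interact"-tagged component touches it and streams the sublevels on either side.
; Timelines drive an optional material fade and button glow, while Door visibility handles open and closed.
; Entering either side volume loads the other side's sublevels; leaving all three door volumes unloads them.
; Construction script builds dynamic materials, positions buttons and gathers sublevel names; IsLocked never gates toggling.
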(event `self.ReceiveBeginPlay`)

(event `TestDoor`
  (`self.ToggleDoorState`))

(event `self.ToggleDoorState`
  (if (not (`self.IsTransitioning`))
    (bind _door_is_open (`self.GetIsOpen`))
    (if _door_is_open
      (`self.Close Door`)
      (else
        (`self.Open Door`)))))

(event `Open Door`
  (`self.Start Button Glow`)
  (set `self.IsTransitioning` true)
  (if (`self.Allow Fade`)
    (bind (_direction _fade_amount) (`Timeline|Door Fade Out` :!via `PlayFromStart`)
      (:`Update`
        (`self.SetFadeOffset` _fade_amount))
      (:`Finished`
        (`SceneComponent.SetVisibility` (`self.Door`) false true :!label _label)
        (set `self.IsOpen` true)
        (set `self.IsTransitioning` false :!label _label_2)))
    (else
      (goto _label))))

(event `Close Door`
  (set `self.IsTransitioning` true)
  (`SceneComponent.SetVisibility` (`self.Door`) true true)
  (if (`self.Allow Fade`)
    (bind (_direction _fade_amount) (`Timeline|Door Fade In` :!via `ReverseFromEnd`)
      (:`Update`
        (`self.SetFadeOffset` _fade_amount))
      (:`Finished`
        (`self.Stop Button Glow` :!label _label_3)
        (set `self.IsOpen` false)
        (goto _label_2)))
    (else
      (goto _label_3))))

(event `self.Touchy.OnComponentBeginOverlap`
  (params (OverlappedComponent :type "PrimitiveComponent Object Reference") (OtherActor :type "Actor Object Reference") (OtherComp :type "PrimitiveComponent Object Reference") (OtherBodyIndex :type Integer) (bFromSweep :type Boolean) (SweepResult :type "HitResult Structure (by ref)"))
  (if (`ActorComponent.ComponentHasTag` OtherComp "Interact")
    (`self.ToggleDoorState`)))

(event `Start Button Glow`
  (bind (_direction _glow_fader) (`Timeline|Button Glow Fade` :!via `PlayFromStart` :!label _label_4)
    (:`Update`
      (`self.SetButtonGlow` _glow_fader))))

(event `Stop Button Glow`
  (goto _label_4 :!via `ReverseFromEnd`))

(event `self.SideA.OnComponentBeginOverlap`
  (params (OverlappedComponent :type "PrimitiveComponent Object Reference") (OtherActor :type "Actor Object Reference") (OtherComp :type "PrimitiveComponent Object Reference") (OtherBodyIndex :type Integer) (bFromSweep :type Boolean) (SweepResult :type "HitResult Structure (by ref)"))
  (if (== OtherActor (`GameplayStatics.GetPlayerPawn` 0))
    (set `self.PlayerInSideA` true)
    (`/Game/Caldoria/Blueprints/BPA_LevelStreamer.Load Sublevel Difference` (`self.BPA_LevelStreamer`) (`self.Side B Sublevel Names`) (`self.Side A Sublevel Names`))))

(event `self.SideA.OnComponentEndOverlap`
  (params (OverlappedComponent :type "PrimitiveComponent Object Reference") (OtherActor :type "Actor Object Reference") (OtherComp :type "PrimitiveComponent Object Reference") (OtherBodyIndex :type Integer))
  (bind _returnvalue (`GameplayStatics.GetPlayerPawn` 0))
  (if (== OtherActor _returnvalue)
    (set `self.PlayerInSideA` (`KismetArrayLibrary.Array_Contains` (`PrimitiveComponent.GetOverlappingActors` OverlappedComponent "/Script/Engine.Pawn") _returnvalue))
    (bind _hethere (`self.PlayerInDoorArea`))
    (if (not _hethere)
      (`/Game/Caldoria/Blueprints/BPA_LevelStreamer.Unload Sublevel Difference` (`self.BPA_LevelStreamer`) (`self.Side A Sublevel Names`) (`self.Side B Sublevel Names`)))))

(event `self.SideB.OnComponentBeginOverlap`
  (params (OverlappedComponent :type "PrimitiveComponent Object Reference") (OtherActor :type "Actor Object Reference") (OtherComp :type "PrimitiveComponent Object Reference") (OtherBodyIndex :type Integer) (bFromSweep :type Boolean) (SweepResult :type "HitResult Structure (by ref)"))
  (if (== OtherActor (`GameplayStatics.GetPlayerPawn` 0))
    (set `self.PlayerInSideB` true)
    (`/Game/Caldoria/Blueprints/BPA_LevelStreamer.Load Sublevel Difference` (`self.BPA_LevelStreamer`) (`self.Side A Sublevel Names`) (`self.Side B Sublevel Names`))))

(event `self.SideB.OnComponentEndOverlap`
  (params (OverlappedComponent :type "PrimitiveComponent Object Reference") (OtherActor :type "Actor Object Reference") (OtherComp :type "PrimitiveComponent Object Reference") (OtherBodyIndex :type Integer))
  (bind _returnvalue (`GameplayStatics.GetPlayerPawn` 0))
  (if (== OtherActor _returnvalue)
    (set `self.PlayerInSideB` (`KismetArrayLibrary.Array_Contains` (`PrimitiveComponent.GetOverlappingActors` OverlappedComponent "/Script/Engine.Pawn") _returnvalue))
    (bind _hethere (`self.PlayerInDoorArea`))
    (if (not _hethere)
      (`/Game/Caldoria/Blueprints/BPA_LevelStreamer.Unload Sublevel Difference` (`self.BPA_LevelStreamer`) (`self.Side B Sublevel Names`) (`self.Side A Sublevel Names`)))))

(event `self.SideInner.OnComponentBeginOverlap`
  (params (OverlappedComponent :type "PrimitiveComponent Object Reference") (OtherActor :type "Actor Object Reference") (OtherComp :type "PrimitiveComponent Object Reference") (OtherBodyIndex :type Integer) (bFromSweep :type Boolean) (SweepResult :type "HitResult Structure (by ref)"))
  (if (== OtherActor (`GameplayStatics.GetPlayerPawn` 0))
    (set `self.PlayerInInner` true)))

(event `self.SideInner.OnComponentEndOverlap`
  (params (OverlappedComponent :type "PrimitiveComponent Object Reference") (OtherActor :type "Actor Object Reference") (OtherComp :type "PrimitiveComponent Object Reference") (OtherBodyIndex :type Integer))
  (bind _returnvalue (`GameplayStatics.GetPlayerPawn` 0))
  (if (== OtherActor _returnvalue)
    (set `self.PlayerInInner` (`KismetArrayLibrary.Array_Contains` (`PrimitiveComponent.GetOverlappingActors` OverlappedComponent "/Script/Engine.Pawn") _returnvalue))))

(event `TestLoadSideA`
  (`/Game/Caldoria/Blueprints/BPA_LevelStreamer.Swap Sublevels` (`self.BPA_LevelStreamer`) (`self.Side A Sublevel Names`) (`self.Side B Sublevel Names`)))

(event `TestLoadSideB`
  (`/Game/Caldoria/Blueprints/BPA_LevelStreamer.Swap Sublevels` (`self.BPA_LevelStreamer`) (`self.Side B Sublevel Names`) (`self.Side A Sublevel Names`)))

(fn `GetIsLocked`
  (returns (IsLocked :type Boolean))
  (return (`self.IsLocked`)))

(fn `GetIsOpen`
  (returns (`Door Is Open` :type Boolean))
  (return (`self.IsOpen`)))

(fn `PlayerInDoorArea`
  (returns (HeThere :type Boolean))
  (return (or (`self.PlayerInSideA`) (`self.PlayerInSideB`) (`self.PlayerInInner`))))

(fn `PopulateLevelDependencies`
  (params (UserWorlds :type "Array of World Soft Object Reference"))
  (returns (Dependencies :type "Set of Name"))
  (locals (NameSet :type "Set of Name"))
  (bind _nameset (`local.NameSet`))
  (for _array_element UserWorlds
    (bind _output (`|ConvertAsset` _array_element))
    (if (`KismetSystemLibrary.IsValid` _output)
      (bind _returnvalue (`KismetStringLibrary.Conv_StringToName` (`KismetSystemLibrary.GetObjectName` _output)))
      (`BlueprintSetLibrary.Set_Add` _nameset _returnvalue)
      (`KismetSystemLibrary.PrintText` (`|FormatText` "Door {door_name}: Added {level_name}" self _returnvalue))))
  (return _nameset))

(fn `SetButtonGlow`
  (params (Amount :type "Float (double-precision)"))
  (`MaterialInstanceDynamic.SetScalarParameterValue` (`self.Instanced Button Material`) "Glow Fader" Amount))

(fn `SetFadeOffset`
  (params (FadeOffset :type "Float (double-precision)"))
  (locals (`Parameter Name` :type Name :default "Fade Offset"))
  (bind _returnvalue (* FadeOffset 2.0))
  (`MaterialInstanceDynamic.SetScalarParameterValue` (`self.Inner Door Dynamic Material`) (`local.Parameter Name`) _returnvalue)
  (`MaterialInstanceDynamic.SetScalarParameterValue` (`self.Outer Door Dynamic Material`) (`local.Parameter Name`) _returnvalue))

(fn `UserConstructionScript`
  (bind _cal_apt_doorway_faaaancy_260x260 (`self.Cal_Apt_Doorway_Faaaancy_260x260`))
  (bind _door (`self.Door`))
  (bind _button_position_offset (`self.Button Position Offset`))
  (bind _returnvalue (* (`self.Button Position Offset`) -1.0))
  (`|ExecutionSequence`
    (:`then_0`
      ;[1 1 1] Setup Materials
      (`PrimitiveComponent.SetMaterial` _cal_apt_doorway_faaaancy_260x260 0 (`self.Inner Wall`))
      (`PrimitiveComponent.SetMaterial` _cal_apt_doorway_faaaancy_260x260 1 (`self.Outer Wall`))
      (bind _returnvalue_2 (`KismetMaterialLibrary.CreateDynamicMaterialInstance` (`self.Inner Door`)))
      (bind _output_get (set `self.Inner Door Dynamic Material` _returnvalue_2))
      (`PrimitiveComponent.SetMaterial` _door 0 _output_get)
      (bind _returnvalue_3 (`KismetMaterialLibrary.CreateDynamicMaterialInstance` (`self.Outer Door`)))
      (bind _output_get_2 (set `self.Outer Door Dynamic Material` _returnvalue_3))
      (`PrimitiveComponent.SetMaterial` _door 1 _output_get_2)
      (bind _returnvalue_4 (`DecalComponent.CreateDynamicMaterialInstance` (`self.Inner Button`)))
      (bind _output_get_3 (set `self.Instanced Button Material` _returnvalue_4))
      (`DecalComponent.SetDecalMaterial` (`self.Outer Button`) _output_get_3))
    (:`then_1`
      (`MaterialInstanceDynamic.SetScalarParameterValue` (`self.Inner Door Dynamic Material`) "Allow Fade" (`KismetMathLibrary.Conv_BoolToDouble` (`self.Allow Fade`)))
      (`MaterialInstanceDynamic.SetScalarParameterValue` (`self.Outer Door Dynamic Material`) "Allow Fade" (`KismetMathLibrary.Conv_BoolToDouble` (`self.Allow Fade`))))
    (:`then_2`
      ;[1 1 1] Set Button Location
      (switch `/Game/Caldoria/Blueprints/Enums/E_Door_Apartment_ButtonSides` (`self.Button Position`)
        (:`NewEnumerator0`
          (`SceneComponent.K2_AddRelativeLocation` (`self.Inner Button`) (`KismetMathLibrary.MakeVector` 0.0 _returnvalue) false false)
          (`SceneComponent.K2_AddRelativeLocation` (`self.Outer Button`) (`KismetMathLibrary.MakeVector` 0.0 _returnvalue) false false))
        (:`NewEnumerator1`
          (`SceneComponent.K2_AddRelativeLocation` (`self.Inner Button`) (`KismetMathLibrary.MakeVector` 0.0 _button_position_offset) false false)
          (`SceneComponent.K2_AddRelativeLocation` (`self.Outer Button`) (`KismetMathLibrary.MakeVector` 0.0 _button_position_offset) false false))))
    (:`then_3`
      (`SceneComponent.SetVisibility` (`self.Door`) (not (`self.IsOpen`)) true))
    (:`then_4`
      (bind _dependencies (`self.PopulateLevelDependencies` (`self.Side A Level`)))
      (set `self.Side A Sublevel Names` _dependencies)
      (bind _dependencies_2 (`self.PopulateLevelDependencies` (`self.Side B Level`)))
      (set `self.Side B Sublevel Names` _dependencies_2))))