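; BP_DeskLamp is a desk lamp that toggles on and off when a component tagged "Interact" touches its button.
; Overlapping ButtonHit sets the bulb to a faint glow, and ending the overlap toggles the lamp.
; On and off switch SpotLight visibility together with the "Bulb Fader" layer parameter on a dynamic material instance.
; The construction script creates that instance and applies the initial IsLit state.
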(event `Toggle Light`
  (if (`self.IsLit`)
    (`self.Turn Light Off`)
    (else
      (`self.Turn Light On`))))

(event `Turn Light On`
  (`SceneComponent.SetVisibility` (`self.SpotLight`) true false)
  (`MaterialInstanceDynamic.SetScalarParameterValueByInfo` (`self.InstancedMaterial`) (`self.Bulb Material Layer`) 1.0)
  (set `self.IsLit` true))

(event `Turn Light Off`
  (`SceneComponent.SetVisibility` (`self.SpotLight`) false false)
  (`MaterialInstanceDynamic.SetScalarParameterValueByInfo` (`self.InstancedMaterial`) (`self.Bulb Material Layer`) 0.0)
  (set `self.IsLit` false))

(event `Struggle Light`
  (`MaterialInstanceDynamic.SetScalarParameterValueByInfo` (`self.InstancedMaterial`) (`self.Bulb Material Layer`) 0.05))

(event `self.Button Hit.OnComponentBeginOverlap`
  (params (OverlappedComponent :type "PrimitiveComponent Object Reference") (OtherActor :type "Actor Object Reference") (OtherComp :type "PrimitiveComponent Object Reference") (OtherBodyIndex :type Integer) (bFromSweep :type Boolean) (SweepResult :type "HitResult Structure (by ref)"))
  (if (`KismetSystemLibrary.IsValid` OtherComp)
    (if (`ActorComponent.ComponentHasTag` OtherComp "Interact")
      (`self.Struggle Light`))))

(event `self.Button Hit.OnComponentEndOverlap`
  (params (OverlappedComponent :type "PrimitiveComponent Object Reference") (OtherActor :type "Actor Object Reference") (OtherComp :type "PrimitiveComponent Object Reference") (OtherBodyIndex :type Integer))
  (if (`KismetSystemLibrary.IsValid` OtherComp)
    (if (`ActorComponent.ComponentHasTag` OtherComp "Interact")
      (`self.Toggle Light`))))

(fn `UserConstructionScript`
  (`|ExecutionSequence`
    (:`then_0`
      (bind _returnvalue (`PrimitiveComponent.CreateDynamicMaterialInstance` (`self.temp_cal_desk_lamp`) 0 null "None"))
      (set `self.InstancedMaterial` _returnvalue)
      (set `self.Bulb Material Layer` (make `MaterialParameterInfo` "Bulb Fader" "LayerParameter" 1)))
    (:`then_2`
      (if (`self.IsLit`)
        (`self.Turn Light On`)
        (else
          (`self.Turn Light Off`))))))