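; Elevator car actor for a VR game that hosts a child-actor keypad and doors and relays their events through dispatcher-style calls.
; Floor requests are passed on, while queue, arrival and door changes update the keypad and its button lights.
; Overlap volumes attach the VR pawn to the floor while inside and report approaching or passed hallway floors.
; A door-blocking volume, active only while doors are open, reports when the player obstructs them.
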(event `self.ReceiveBeginPlay`
  (`self.Setup Keypad`)
  (`self.Setup Elevator Doors`))

(event `self.Detect Player.OnComponentBeginOverlap`
  (params (OverlappedComponent :type "PrimitiveComponent Object Reference") (OtherActor :type "Actor Object Reference") (OtherComp :type "PrimitiveComponent Object Reference") (OtherBodyIndex :type Integer) (bFromSweep :type Boolean) (SweepResult :type "HitResult Structure (by ref)"))
  (bind _asvrpawn_agent_5 (cast `/Game/_Player/VRPawn_Agent5` OtherActor))
  (`self.K2_AttachToComponent` _asvrpawn_agent_5 (`self.Floor`) "None" "KeepWorld" "KeepWorld" "KeepWorld" true)
  (set `self.PlayerInside` true)
  (`self.Player Entered`)
  (`KismetSystemLibrary.PrintString` "Player Attatched To Car"))

(event `self.Detect Player.OnComponentEndOverlap`
  (params (OverlappedComponent :type "PrimitiveComponent Object Reference") (OtherActor :type "Actor Object Reference") (OtherComp :type "PrimitiveComponent Object Reference") (OtherBodyIndex :type Integer))
  (bind _asvrpawn_agent_5 (cast `/Game/_Player/VRPawn_Agent5` OtherActor))
  (`self.K2_DetachFromActor` _asvrpawn_agent_5 "KeepWorld" "KeepWorld" "KeepWorld")
  (set `self.PlayerInside` false)
  (`self.Player Exited`)
  (`KismetSystemLibrary.PrintString` "Player detatched from car"))

(event `Keypad Requested Floor`
  (params (`Requested Floor` :type "/Game/Caldoria/Blueprints/BP_Elevator_Hallway Object Reference"))
  (`self.Floor Requested` `Requested Floor`))

(event `Floor Added To Queue`
  (params (`Queued Floor` :type "/Game/Caldoria/Blueprints/BP_Elevator_Hallway Object Reference"))
  (`/Game/Caldoria/Blueprints/BP_Elevator_Keypad.Floor Added To Queue` (`self.Instanced Keypad`) `Queued Floor`))

(event `Floor Removed From Queue`
  (params (`Removed Floor` :type "/Game/Caldoria/Blueprints/BP_Elevator_Hallway Object Reference"))
  (`/Game/Caldoria/Blueprints/BP_Elevator_Keypad.Floor Removed From Queue` (`self.Instanced Keypad`) `Removed Floor`))

(event `Arrived At Floor`
  (params (`At Floor` :type "/Game/Caldoria/Blueprints/BP_Elevator_Hallway Object Reference"))
  (set `self.Current Floor` `At Floor`))

(event `Leaving Floor`
  (params (Floor :type "/Game/Caldoria/Blueprints/BP_Elevator_Hallway Object Reference"))
  (bind _keypad_button (`/Game/Caldoria/Blueprints/BP_Elevator_Keypad.GetButtonForFloor` (`self.Instanced Keypad`) Floor))
  (`/Game/Caldoria/Blueprints/BP_Elevator_Keypad_Button.TurnButtonOff` _keypad_button)
  (set `self.Current Floor` null))

(event `self.WatchYourFingies.OnComponentBeginOverlap`
  (params (OverlappedComponent :type "PrimitiveComponent Object Reference") (OtherActor :type "Actor Object Reference") (OtherComp :type "PrimitiveComponent Object Reference") (OtherBodyIndex :type Integer) (bFromSweep :type Boolean) (SweepResult :type "HitResult Structure (by ref)"))
  (cast `/Game/_Player/VRPawn_Agent5` OtherActor)
  (`self.Player Blocking Door` true))

(event `self.WatchYourFingies.OnComponentEndOverlap`
  (params (OverlappedComponent :type "PrimitiveComponent Object Reference") (OtherActor :type "Actor Object Reference") (OtherComp :type "PrimitiveComponent Object Reference") (OtherBodyIndex :type Integer))
  (cast `/Game/_Player/VRPawn_Agent5` OtherActor)
  (`self.Player Blocking Door` false))

(event `Test Open Doors`
  (`self.Open Doors` 5.0))

(event `Test Close Doors`
  (`self.Close Doors` 0.0))

(event `Open Doors`
  (params (`Open Rate` :type "Float (double-precision)" :default 5.0))
  (`/Game/Caldoria/Blueprints/BP_Elevator_Doors.Open Doors` (`self.Instanced Elevator Doors`) `Open Rate`)
  (if (`KismetSystemLibrary.IsValid` (`self.Current Floor`))
    (bind _keypad_button (`/Game/Caldoria/Blueprints/BP_Elevator_Keypad.GetButtonForFloor` (`self.Instanced Keypad`) (`self.Current Floor`)))
    (`/Game/Caldoria/Blueprints/BP_Elevator_Keypad_Button.TurnButtonOn` _keypad_button true)))

(event `Close Doors`
  (params (`Close Rate` :type "Float (double-precision)"))
  (`/Game/Caldoria/Blueprints/BP_Elevator_Doors.Close Doors` (`self.Instanced Elevator Doors`) `Close Rate`))

(event `Door State Changed`
  (params (`Doors Are Open` :type Boolean))
  (`self.Doors State Changed` `Doors Are Open`)
  (if `Doors Are Open`
    (`PrimitiveComponent.SetCollisionEnabled` (`self.WatchYourFingies`) (`self.FingieCollisionType`))
    (else
      (`PrimitiveComponent.SetCollisionEnabled` (`self.WatchYourFingies`) "NoCollision")
      (if (`KismetSystemLibrary.IsValid` (`self.Current Floor`))
        (bind _keypad_button (`/Game/Caldoria/Blueprints/BP_Elevator_Keypad.GetButtonForFloor` (`self.Instanced Keypad`) (`self.Current Floor`)))
        (`/Game/Caldoria/Blueprints/BP_Elevator_Keypad_Button.TurnButtonOff` _keypad_button)))))

(event `self.Detect Floor.OnComponentBeginOverlap`
  (params (OverlappedComponent :type "PrimitiveComponent Object Reference") (OtherActor :type "Actor Object Reference") (OtherComp :type "PrimitiveComponent Object Reference") (OtherBodyIndex :type Integer) (bFromSweep :type Boolean) (SweepResult :type "HitResult Structure (by ref)"))
  (if (`ActorComponent.ComponentHasTag` OtherComp "Floor Notifier")
    (bind _asbp_elevator_hallway (cast `/Game/Caldoria/Blueprints/BP_Elevator_Hallway` OtherActor))
    (`self.Car Approaching Floor` _asbp_elevator_hallway)
    (`KismetSystemLibrary.PrintText` (`|FormatText` "Elevator approaching Floor {number}" (`/Game/Caldoria/Blueprints/BP_Elevator_Hallway.Floor Number` _asbp_elevator_hallway)))))

(event `self.Detect Floor.OnComponentEndOverlap`
  (params (OverlappedComponent :type "PrimitiveComponent Object Reference") (OtherActor :type "Actor Object Reference") (OtherComp :type "PrimitiveComponent Object Reference") (OtherBodyIndex :type Integer))
  (if (`ActorComponent.ComponentHasTag` OtherComp "Floor Notifier")
    (bind _asbp_elevator_hallway (cast `/Game/Caldoria/Blueprints/BP_Elevator_Hallway` OtherActor))
    (`self.Car Passed By Floor` _asbp_elevator_hallway)
    (`KismetSystemLibrary.PrintText` (`|FormatText` "Elevator leaving Floor {number}" (`/Game/Caldoria/Blueprints/BP_Elevator_Hallway.Floor Number` _asbp_elevator_hallway)))))

(fn `AddFloorToList`
  (params (`New Floor` :type "/Game/Caldoria/Blueprints/BP_Elevator_Hallway Object Reference"))
  (`/Game/Caldoria/Blueprints/BP_Elevator_Keypad.Add Floor Button` (`self.Instanced Keypad`) `New Floor` "NewEnumerator0"))

(fn `Setup Elevator Doors`
  (`|ExecutionSequence`
    (:`then_0`
      (bind _asbp_elevator_doors (cast `/Game/Caldoria/Blueprints/BP_Elevator_Doors` (`ChildActorComponent.ChildActor` (`self.BP_Elevator_Doors`))))
      (set `self.Instanced Elevator Doors` _asbp_elevator_doors))
    (:`then_1`
      (add `/Game/Caldoria/Blueprints/BP_Elevator_Doors.DoorStateChanged` (`self.Instanced Elevator Doors`) (`|CreateDelegate` :!event `Door State Changed`)))))

(fn `Setup Keypad`
  (`|ExecutionSequence`
    (:`then_0`
      (bind _asbp_elevator_keypad (cast `/Game/Caldoria/Blueprints/BP_Elevator_Keypad` (`ChildActorComponent.ChildActor` (`self.BP_Elevator_Keypad`))))
      (set `self.Instanced Keypad` _asbp_elevator_keypad))
    (:`then_1`
      (add `/Game/Caldoria/Blueprints/BP_Elevator_Keypad.FloorRequested` (`self.Instanced Keypad`) (`|CreateDelegate` :!event `Keypad Requested Floor`)))))

(fn `UserConstructionScript`
  (bind _watchyourfingies (`self.WatchYourFingies`))
  (`|ExecutionSequence`
    (:`then_0`
      (set `self.FingieCollisionType` (`PrimitiveComponent.GetCollisionEnabled` _watchyourfingies))
      (`PrimitiveComponent.SetCollisionEnabled` _watchyourfingies "NoCollision"))))