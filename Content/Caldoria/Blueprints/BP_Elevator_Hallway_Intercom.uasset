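; Elevator hallway intercom with a call button that lights up or pulses and a speaker that plays a supplied sound.
; Setup caches a spring-loaded button child actor, gives it a dynamic material and timeout, and binds its press, which is relayed through the CallButtonPressed dispatcher.
; Timelines fade the glow on and off through material parameters, guarded by lit and transition flags.
; Debug prints report audio and press activity.
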(event `self.ReceiveBeginPlay`
  (bind _audio (`self.Audio`))
  (`self.Setup Button`)
  (add `AudioComponent.OnAudioPlayStateChanged` _audio (delegate `CustomEvent`))
  (`KismetSystemLibrary.PrintString` (`KismetSystemLibrary.GetDisplayName` (`AudioComponent.Sound` _audio))))

(event `CustomEvent`
  (params (PlayState :type "EAudioComponentPlayState Enum" :default "Playing"))
  (`KismetSystemLibrary.PrintString` (`|GetEnumeratorNameAsString` PlayState)))

(event `Illuminate Button`
  (params (Flashing :type Boolean))
  (`self.Set Is Flashing` Flashing)
  (if (`self.ButtonIsTransitioning`)
    _
    (elif (not (`self.IsLit`))
      (set `self.ButtonIsTransitioning` true)
      (bind (_direction _glow_amount) (`Timeline|Timeline` :!via `PlayFromStart`)
        (:`Update`
          (`self.Set Button Glow` _glow_amount))
        (:`Finished`
          (set `self.ButtonIsTransitioning` false)
          (set `self.IsLit` true))))))

(event `Turn Off Light`
  (if (`self.ButtonIsTransitioning`)
    _
    (elif (`self.IsLit`)
      (set `self.ButtonIsTransitioning` true)
      (`TimelineComponent.SetPlayRate` (`self.Timeline_0`) 2.0)
      (bind (_direction _glow_amount) (`Timeline|Timeline_0` :!via `PlayFromStart`)
        (:`Update`
          (`self.Set Button Glow` (- 1.0 _glow_amount))
          (`self.Set Is Flashing` false)
          (set `self.ButtonIsTransitioning` false)
          (set `self.IsLit` false))))))

(event `Button Was Pressed`
  (`self.Call Button Pressed`)
  (`KismetSystemLibrary.PrintString` "Hello"))

(fn `Set Button Glow`
  (params (`Glow Amount` :type "Float (double-precision)"))
  (`MaterialInstanceDynamic.SetScalarParameterValue` (`self.Instanced Button Material`) "Glow Fade" `Glow Amount`))

(fn `Set Is Flashing`
  (params (`Is Flashing` :type Boolean))
  (`MaterialInstanceDynamic.SetScalarParameterValue` (`self.Instanced Button Material`) "Is Pulsing" (`KismetMathLibrary.Conv_BoolToDouble` `Is Flashing`)))

(fn `Set Speaker Audio`
  (params (`Audio Source` :type "SoundBase Object Reference"))
  (bind _audio (`self.Audio`))
  (`AudioComponent.SetSound` _audio `Audio Source`)
  (`AudioComponent.Play` _audio 0.0))

(fn `Setup Button`
  (bind _instanced_button (`self.Instanced Button`))
  (`|ExecutionSequence`
    (:`then_0`
      (bind _asbp_spring_loaded_button (cast `/Game/Caldoria/Blueprints/BP_SpringLoadedButton` (`ChildActorComponent.ChildActor` (`self.BP_SpringLoadedButton`))))
      (set `self.Instanced Button` _asbp_spring_loaded_button))
    (:`then_1`
      (bind _button_component (`/Game/Caldoria/Blueprints/BP_SpringLoadedButton.Get Button Component` _instanced_button))
      (bind _returnvalue (`PrimitiveComponent.CreateDynamicMaterialInstance` _button_component 0 null "None"))
      (set `self.Instanced Button Material` _returnvalue))
    (:`then_2`
      (set `/Game/Caldoria/Blueprints/BP_SpringLoadedButton.Timeout Duration (Seconds)` (`self.Button Timeout Duration (s)`) _instanced_button))
    (:`then_3`
      (add `/Game/Caldoria/Blueprints/BP_SpringLoadedButton.ButtonPressed` _instanced_button (`|CreateDelegate` :!event `Button Was Pressed`)))))

(fn `UserConstructionScript`)