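; Sliding, lockable apartment hallway door that streams the levels outside it, loading them as it opens and unloading them once it has closed.
; An Interact-tagged overlap toggles timeline-driven door motion and button glow, or plays the intercom message if locked.
; BeginPlay configures the child-actor intercom's message and binds its button events, with ding/dong doorbell audio triggers.
; The construction script applies apartment number, materials and movement rate.
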(event `self.ReceiveBeginPlay`
  (`self.Setup Intercom`)
  (`self.Setup Doorbell`))

(event `TestDoorOpener`
  (`/Game/Caldoria/Blueprints/BPI_Door.ToggleDoorState`))

(event `Lock Door`
  (params (LockDoor :type Boolean))
  (set `self.IsLocked` LockDoor))

(event `Open Door`
  (if (`self.IsTransitioning`)
    _
    (elif (not (`self.IsLocked`))
      (`/Game/Caldoria/Blueprints/BPA_LevelStreamer.Load Sublevels` (`self.BPA_LevelStreamer`) (`self.Outside Level Names`))
      (set `self.IsTransitioning` true)
      (`self.Start Button Glow`)
      (bind (_direction _newtrack_0) (`Timeline|Door Offset Opening` :!via `PlayFromStart`)
        (:`Update`
          (`SceneComponent.K2_SetRelativeLocation` (`self.Door`) (`KismetMathLibrary.MakeVector` 0.0 (* _newtrack_0 (`self.Door Width`))) false false))
        (:`Finished`
          (set `self.IsOpen` true)
          (set `self.IsTransitioning` false :!label _label))))))

(event `Close Door`
  (bind _door_width (`self.Door Width`))
  (if (not (`self.IsTransitioning`))
    (set `self.IsTransitioning` true)
    (bind (_direction _newtrack_0) (`Timeline|Door Offset Closing` :!via `PlayFromStart`)
      (:`Update`
        (`SceneComponent.K2_SetRelativeLocation` (`self.Door`) (`KismetMathLibrary.MakeVector` 0.0 (- _door_width (* _newtrack_0 _door_width))) false false))
      (:`Finished`
        (`self.Stop Button Glow`)
        (`/Game/Caldoria/Blueprints/BPA_LevelStreamer.Unload Sublevels` (`self.BPA_LevelStreamer`) (`self.Outside Level Names`))
        (set `self.IsOpen` false)
        (goto _label)))))

(event `/Game/Caldoria/Blueprints/BPI_Door.ToggleDoorState`
  (if (`self.IsOpen`)
    (`self.Close Door`)
    (elif (`self.IsLocked`)
      (`/Game/Caldoria/Blueprints/BP_Door_Intercom.Play Message` (`self.InstancedIntercom`))
      (else
        (`self.Open Door`)))))

(event `self.Touchy.OnComponentBeginOverlap`
  (params (OverlappedComponent :type "PrimitiveComponent Object Reference") (OtherActor :type "Actor Object Reference") (OtherComp :type "PrimitiveComponent Object Reference") (OtherBodyIndex :type Integer) (bFromSweep :type Boolean) (SweepResult :type "HitResult Structure (by ref)"))
  (if (`ActorComponent.ComponentHasTag` OtherComp "Interact")
    (`/Game/Caldoria/Blueprints/BPI_Door.ToggleDoorState`)))

(event `Start Button Glow`
  (bind (_direction _glow_fader) (`Timeline|Button Glow In` :!via `PlayFromStart` :!label _label_2)
    (:`Update`
      (`self.Set Button Glow` _glow_fader)
      (`/Game/Caldoria/Blueprints/BP_Door_Intercom.Set Glow Intensity` (`self.InstancedIntercom`) _glow_fader))))

(event `Stop Button Glow`
  (goto _label_2 :!via `ReverseFromEnd`))

(event `Doorbell Bing`
  (`AudioParameterControllerInterface.SetTriggerParameter` (`self.Doorbell Emitter`) "Play Ding"))

(event `Doorbell Bong`
  (`AudioParameterControllerInterface.SetTriggerParameter` (`self.Doorbell Emitter`) "Play Dong"))

(fn `GetIsLocked`
  (returns (IsLocked :type Boolean))
  (return (`self.IsLocked`)))

(fn `GetIsOpen`
  (returns (`Door Is Open` :type Boolean))
  (return (`self.IsOpen`)))

(fn `Set Button Glow`
  (params (Amount :type "Float (double-precision)"))
  (`MaterialInstanceDynamic.SetScalarParameterValue` (`self.Dynamic Button Material`) "Glow Fader" Amount))

(fn `Setup Doorbell`
  (bind _instancedintercom (`self.InstancedIntercom`))
  (add `/Game/Caldoria/Blueprints/BP_Door_Intercom.ButtonPressed` _instancedintercom (`|CreateDelegate` :!event `Doorbell Bing`))
  (add `/Game/Caldoria/Blueprints/BP_Door_Intercom.ButtonUnPressed` _instancedintercom (`|CreateDelegate` :!event `Doorbell Bong`)))

(fn `Setup Intercom`
  (`|ExecutionSequence`
    (:`then_0`
      (bind _asbp_door_intercom (cast `/Game/Caldoria/Blueprints/BP_Door_Intercom` (`ChildActorComponent.ChildActor` (`self.BP_Door_Intercom`))))
      (set `self.InstancedIntercom` _asbp_door_intercom))
    (:`then_1`
      (`/Game/Caldoria/Blueprints/BP_Door_Intercom.Set Message` (`self.InstancedIntercom`) (`self.Message`)))
    (:`then_2`
      (add `/Game/Caldoria/Blueprints/BP_Door_Intercom.ButtonUnPressed` (`self.InstancedIntercom`) (`|CreateDelegate` :!event `ToggleDoorState`)))))

(fn `UserConstructionScript`
  (bind _door_movement_rate (`self.Door Movement Rate`))
  (`|ExecutionSequence`
    (:`then_0`
      ;[1 1 1] Apartment Number
      (`TextRenderComponent.K2_SetText` (`self.AptNumberText`) (`self.ApartmentNumber`)))
    (:`then_1`
      ;[1 1 1] Material Setup
      (`PrimitiveComponent.SetMaterial` (`self.Door`) 1 (`self.Outer Door`))
      (`PrimitiveComponent.SetMaterial` (`self.Door`) 0 (`self.Inner Door`))
      (`PrimitiveComponent.SetMaterial` (`self.Cal_Apt_Doorway_Faaaancy_260x260`) 1 (`self.Inner Wall`))
      (`PrimitiveComponent.SetMaterial` (`self.Cal_Apt_Doorway_Faaaancy_260x260`) 0 (`self.Outer Wall`))
      (bind _returnvalue (`DecalComponent.CreateDynamicMaterialInstance` (`self.Inner Button`)))
      (set `self.Dynamic Button Material` _returnvalue))
    (:`then_2`
      ;[1 1 1] Set Timeline Playback Rates
      (`TimelineComponent.SetPlayRate` (`self.Door Offset Opening`) _door_movement_rate)
      (`TimelineComponent.SetPlayRate` (`self.Door Offset Closing`) _door_movement_rate))))