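; Elevator controller for the Caldoria level that runs one child-actor car between registered floors and coordinates car and hallway doors.
; Car and floor requests feed a first-in, first-out queue, served once the car is idle and doors are closed.
; Timelines move the car with a starting dip and distance-scaled play rate; arrival opens doors on an auto-close timer, extended by player blocking.
; Approach and pass events stream hallway sublevels by floor-number name.
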(event `self.ReceiveBeginPlay`
  (`self.Setup Elevator Car`)
  (`self.Setup Floor Database`))

(event `Floor Added To Directory`
  (params (`New Floor` :type "/Game/Caldoria/Blueprints/BP_Elevator_Hallway Object Reference"))
  (add `/Game/Caldoria/Blueprints/BP_Elevator_Hallway.Floor Requested` `New Floor` (delegate `Floor Requested`))
  (`/Game/Caldoria/Blueprints/BP_Elevator_Car.AddFloorToList` (`self.Instanced Elevator Car`) `New Floor`))

(event `Floor Requested`
  (params (`Requested Floor` :type "/Game/Caldoria/Blueprints/BP_Elevator_Hallway Object Reference"))
  (`KismetSystemLibrary.PrintString` (`KismetTextLibrary.Conv_TextToString` (`|FormatText` "Calling floor {floor_index}" (`/Game/Caldoria/Blueprints/BP_Elevator_Hallway.Floor Number` `Requested Floor`))))
  (bind _was_added (`self.Add Floor To Queue` `Requested Floor`))
  (if _was_added
    (`/Game/Caldoria/Blueprints/BP_Elevator_Hallway.Floor Added To Queue` `Requested Floor`)
    (`/Game/Caldoria/Blueprints/BP_Elevator_Car.Floor Added To Queue` (`self.Instanced Elevator Car`) `Requested Floor`))
  (`self.Next In Queue`))

(event `Move Car To Floor`
  (params (`Destination Floor` :type "/Game/Caldoria/Blueprints/BP_Elevator_Hallway Object Reference"))
  (bind _instanced_elevator_car (`self.Instanced Elevator Car`))
  (bind _instanced_elevator_car_2 (`self.Instanced Elevator Car`))
  (bind (_returnvalue_x _returnvalue_y _returnvalue_z) (`KismetMathLibrary.BreakVector` (`self.K2_GetActorLocation` _instanced_elevator_car_2)))
  (bind (_returnvalue_x_2 _returnvalue_y_2 _returnvalue_z_2) (`KismetMathLibrary.BreakVector` (`self.K2_GetActorLocation` _instanced_elevator_car)))
  (set `self.CarIsTraveling` true)
  (bind _z_distance_to_floor (`self.GetDistanceToTravel` `Destination Floor`))
  (`TimelineComponent.SetPlayRate` (`self.Car Mover`) (`KismetMathLibrary.Abs` (/ (`self.Car Rate`) _z_distance_to_floor)))
  ;[1 1 1] Dip Animation Attempt
  (`TimelineComponent.SetPlayRate` (`self.Car Mover Dip Down`) (/ (`self.Car Rate`) 40.0))
  (bind _output_get (set `self.Car Initial Z` _returnvalue_z_2))
  (bind (_direction _dip) (`Timeline|Car Mover Dip Down` :!via `PlayFromStart`)
    (:`Update`
      (`self.K2_SetActorLocation` _instanced_elevator_car (`KismetMathLibrary.MakeVector` _returnvalue_x_2 _returnvalue_y_2 (+ (* _dip 1.0) _output_get)) false false))
    (:`Finished`
      (bind _output_get_2 (set `self.Car Initial Z` _returnvalue_z))
      (bind (_direction_2 _z_change) (`Timeline|Car Mover` :!via `PlayFromStart`)
        (:`Update`
          (`self.K2_SetActorLocation` _instanced_elevator_car_2 (`KismetMathLibrary.MakeVector` _returnvalue_x _returnvalue_y (+ (`KismetMathLibrary.Lerp` 0.0 _z_distance_to_floor _z_change) _output_get_2)) false false))
        (:`Finished`
          (`KismetSystemLibrary.Delay` (`self.Safety Delay`))
          (set `self.CarIsTraveling` false)
          (`self.Arrived At Floor` `Destination Floor`))))))

(event `Car Approaching Floor`
  (params (`Incoming Floor` :type "/Game/Caldoria/Blueprints/BP_Elevator_Hallway Object Reference"))
  (bind _hallway_sublevel_name (`self.Build Hallway Sublevel Name` `Incoming Floor`))
  (`/Game/Caldoria/Blueprints/BPA_LevelStreamer.Load Sublevel` (`self.BPA_LevelStreamer`) _hallway_sublevel_name))

(event `Car Passed Floor`
  (params (`Outgoing Floor` :type "/Game/Caldoria/Blueprints/BP_Elevator_Hallway Object Reference"))
  (bind _hallway_sublevel_name (`self.Build Hallway Sublevel Name` `Outgoing Floor`))
  (`/Game/Caldoria/Blueprints/BPA_LevelStreamer.Unload Sublevel` (`self.BPA_LevelStreamer`) _hallway_sublevel_name))

(event `Arrived At Floor`
  (params (`At Floor` :type "/Game/Caldoria/Blueprints/BP_Elevator_Hallway Object Reference"))
  (`self.RemoveFloorFromQueue` `At Floor`)
  (bind _output_get (set `self.CurrentFloor` `At Floor`))
  (`/Game/Caldoria/Blueprints/BP_Elevator_Car.Arrived At Floor` (`self.Instanced Elevator Car`) _output_get) ; Let the Car know
  (`self.Open Doors` true))

(event `Next In Queue`
  (if (`self.CarIsTraveling`)
    _
    (elif (not (`self.DoorsAreOpen`))
      (bind (_next_floor _has_floor_in_queue) (`self.GetNextFloorInQueue`))
      (if _has_floor_in_queue
        (if (== _next_floor (`self.CurrentFloor`))
          (`self.Arrived At Floor` _next_floor)
          (else
            (`self.Move Car To Floor` _next_floor)))))))

(event `Test Player Blocked Door`
  (`self.Player Blocked Door` true))

(event `Open Doors`
  (params (`Set Close Timer` :type Boolean :default true))
  (bind _door_open_rate (`self.Door Open Rate`))
  (bind _door_close_timer (`self.Door Close Timer`))
  (bind _door_random_rate_range__dr3_ (`self.Door Random Rate Range (DR3)`))
  (bind _returnvalue (- _door_random_rate_range__dr3_ (/ _door_random_rate_range__dr3_ 2.0)))
  (if (`KismetSystemLibrary.K2_IsValidTimerHandle` _door_close_timer)
    (`KismetSystemLibrary.K2_ClearAndInvalidateTimerHandle` _door_close_timer))
  (`/Game/Caldoria/Blueprints/BP_Elevator_Hallway.Open Doors` (`self.CurrentFloor`) _door_open_rate)
  (`/Game/Caldoria/Blueprints/BP_Elevator_Car.Open Doors` (`self.Instanced Elevator Car`) (+ _door_open_rate (`KismetMathLibrary.RandomFloatInRange` (* _returnvalue -1.0) _returnvalue)))
  (`KismetSystemLibrary.Delay` 0.5)
  ;[1 1 1] Need Callback for After Doors Are Open?
  (if `Set Close Timer`
    (bind _returnvalue_2 (`KismetSystemLibrary.K2_SetTimerDelegate` (`|CreateDelegate` :!event `Close Doors`) 5.0))
    (set `self.Door Close Timer` _returnvalue_2)))

(event `Test Player Unblocked Door`
  (`self.Player Blocked Door` false))

(event `Test Open Doors`
  (`self.Open Doors` true))

(event `Close Doors`
  (bind _door_open_rate (`self.Door Open Rate`))
  (bind _door_random_rate_range__dr3_ (`self.Door Random Rate Range (DR3)`))
  (bind _returnvalue (- _door_random_rate_range__dr3_ (/ _door_random_rate_range__dr3_ 2.0)))
  (`/Game/Caldoria/Blueprints/BP_Elevator_Hallway.Close Doors` (`self.CurrentFloor`) _door_open_rate)
  (`/Game/Caldoria/Blueprints/BP_Elevator_Car.Close Doors` (`self.Instanced Elevator Car`) (+ (`KismetMathLibrary.RandomFloatInRange` (* _returnvalue -1.0) _returnvalue) _door_open_rate)))

(event `Test Next Floor`
  (`self.Next In Queue`))

(event `Door State Changed`
  (params (`Doors Are Open` :type Boolean))
  (bind _output_get (set `self.DoorsAreOpen` `Doors Are Open`))
  (if (not _output_get)
    (`KismetSystemLibrary.Delay` (`self.Safety Delay`))
    (`self.Next In Queue`)))

(event `Player Blocked Door`
  (params (`Is Blocking` :type Boolean))
  (bind _door_is_open (`/Game/Caldoria/Blueprints/BPI_Door.GetIsOpen` (`self.CurrentFloor`)))
  (if _door_is_open
    (if `Is Blocking`
      (`self.Open Doors` false :!label _label)
      (else
        (`self.Open Doors` true)))
    (elif `Is Blocking`
      (goto _label))))

(fn `Add Floor`
  (params (Floor :type "/Game/Caldoria/Blueprints/BP_Elevator_Hallway Object Reference"))
  (bind _floor_list (`self.Floor List`))
  (if (not (`BlueprintSetLibrary.Set_Contains` _floor_list Floor))
    (`BlueprintSetLibrary.Set_Add` _floor_list Floor)
    (`self.Floor Added To Directory` Floor)
    ;[1 1 1] Debug
    (`KismetSystemLibrary.PrintText` (`|FormatText` "Floor {floor_index} has been added to the database" (`KismetTextLibrary.Conv_StringToText` (`/Game/Caldoria/Blueprints/BP_Elevator_Hallway.Floor Number` Floor))))))

(fn `Add Floor To Queue`
  (params (Floor :type "/Game/Caldoria/Blueprints/BP_Elevator_Hallway Object Reference"))
  (returns (`Was Added` :type Boolean))
  (bind _active_queue (`self.Active Queue`))
  (if (`KismetArrayLibrary.Array_Contains` _active_queue Floor)
    (`KismetSystemLibrary.PrintText` (`|FormatText` "Floor {floor_number} already in queue" (`/Game/Caldoria/Blueprints/BP_Elevator_Hallway.Floor Number` Floor)))
    (return false)
    (else
      (`KismetArrayLibrary.Array_Add` _active_queue Floor)
      (`KismetSystemLibrary.PrintText` (`|FormatText` "Floor {floor_number} added to queue" (`/Game/Caldoria/Blueprints/BP_Elevator_Hallway.Floor Number` Floor)))
      (return true))))

(fn `Build Hallway Sublevel Name`
  (params (Floor :type "/Game/Caldoria/Blueprints/BP_Elevator_Hallway Object Reference (by ref)"))
  (returns (`Hallway Sublevel Name` :type Name))
  (return (`KismetStringLibrary.Conv_StringToName` (`KismetTextLibrary.Conv_TextToString` (`|FormatText` "L_Caldoria_{Floor Number}_Hallway" (`/Game/Caldoria/Blueprints/BP_Elevator_Hallway.Floor Number` Floor))))))

(fn `GetDistanceToTravel`
  (params (`Destination Floor` :type "/Game/Caldoria/Blueprints/BP_Elevator_Hallway Object Reference"))
  (returns (`Z Distance To Floor` :type "Float (double-precision)"))
  (bind (_returnvalue_x _returnvalue_y _returnvalue_z) (`KismetMathLibrary.BreakVector` (`self.K2_GetActorLocation` `Destination Floor`)))
  (bind (_returnvalue_x_2 _returnvalue_y_2 _returnvalue_z_2) (`KismetMathLibrary.BreakVector` (`self.K2_GetActorLocation` (`self.Instanced Elevator Car`))))
  (return (- _returnvalue_z _returnvalue_z_2)))

(fn `GetNextFloorInQueue`
  (returns (`Next Floor` :type "/Game/Caldoria/Blueprints/BP_Elevator_Hallway Object Reference") (`Has Floor In Queue` :type Boolean))
  (bind _active_queue (`self.Active Queue`))
  (if (`KismetArrayLibrary.Array_IsEmpty` _active_queue)
    (return null false)
    (else
      (return (`|GetArrayItem` _active_queue) true))))

(fn `RemoveFloorFromQueue`
  (params (`Floor to Remove` :type "/Game/Caldoria/Blueprints/BP_Elevator_Hallway Object Reference"))
  (returns (`Was Removed` :type Boolean))
  (bind _returnvalue (`KismetArrayLibrary.Array_RemoveItem` (`self.Active Queue`) `Floor to Remove`))
  (`self.Floor Removed From Queue` `Floor to Remove`)
  (return _returnvalue))

(fn `Setup Elevator Car`
  (bind _instanced_elevator_car (`self.Instanced Elevator Car`))
  (`|ExecutionSequence`
    (:`then_0`
      (bind _asbp_elevator_car (cast `/Game/Caldoria/Blueprints/BP_Elevator_Car` (`ChildActorComponent.ChildActor` (`self.BP_Elevator_Car`))))
      (set `self.Instanced Elevator Car` _asbp_elevator_car))
    (:`then_1`
      (add `/Game/Caldoria/Blueprints/BP_Elevator_Car.Floor Requested` _instanced_elevator_car (`|CreateDelegate` :!event `Floor Requested`))
      (add `/Game/Caldoria/Blueprints/BP_Elevator_Car.Player Blocking Door` _instanced_elevator_car (`|CreateDelegate` :!event `Player Blocked Door`))
      (add `/Game/Caldoria/Blueprints/BP_Elevator_Car.Doors State Changed` _instanced_elevator_car (`|CreateDelegate` :!event `Door State Changed`))
      (add `/Game/Caldoria/Blueprints/BP_Elevator_Car.Car Approaching Floor` _instanced_elevator_car (`|CreateDelegate` :!event `Car Approaching Floor`))
      (add `/Game/Caldoria/Blueprints/BP_Elevator_Car.Car Passed By Floor` _instanced_elevator_car (`|CreateDelegate` :!event `Car Passed Floor`)))))

(fn `Setup Floor Database`
  (for _array_element (`self.Floors`)
    (`self.Add Floor` _array_element)))

(fn `UserConstructionScript`
  (`|ExecutionSequence`))