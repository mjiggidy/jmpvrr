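; BP_Elevator_Hallway is the hallway side of an elevator stop, with a call intercom, doors and a floor-number sign.
; BeginPlay caches the intercom and door child actors and binds the call button; floor requests go out through the CallFloorRequested dispatcher.
; Queue and open/close events drive the intercom lights and delegate movement to the doors actor.
; The construction script sets the sign decal's dynamic material from the floor number, using a lookup for non-numeric floors.
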(event `Request This Floor`
  (`self.Floor Requested` self))

(event `self.ReceiveBeginPlay`
  (`self.Setup Intercom`)
  (`self.Setup Elevator Doors`))

(event `Test Floor Requested`
  (`self.Floor Requested` self))

(event `Floor Added To Queue`
  (`/Game/Caldoria/Blueprints/BP_Elevator_Hallway_Intercom.Illuminate Button` (`self.Instanced Elevator Intercom`) false))

(event `Arrived At Floor`)

(event `Test Open Doors`
  (`self.Open Doors` 1.0))

(event `Test Close Doors`
  (`self.Close Doors` 1.0))

(event `Open Doors`
  (params (`Open Rate` :type "Float (double-precision)" :default 1.0))
  (`/Game/Caldoria/Blueprints/BP_Elevator_Hallway_Intercom.Illuminate Button` (`self.Instanced Elevator Intercom`) true)
  (`/Game/Caldoria/Blueprints/BP_Elevator_Doors.Open Doors` (`self.Instanced Elevator Doors`) `Open Rate`))

(event `Close Doors`
  (params (`Close Rate` :type "Float (double-precision)" :default 1.0))
  (`/Game/Caldoria/Blueprints/BP_Elevator_Doors.Close Doors` (`self.Instanced Elevator Doors`) `Close Rate`)
  (`/Game/Caldoria/Blueprints/BP_Elevator_Hallway_Intercom.Turn Off Light` (`self.Instanced Elevator Intercom`)))

(fn `FloorIndexFromNumber`
  (params (`Floor Number` :type String))
  (returns (`Floor Index` :type "Float (double-precision)"))
  (locals (`Special Lookup` :type "Map of String to Float (double-precision)") (Unknown :type "Float (double-precision)" :default 6.0))
  (bind (_value _returnvalue) (`BlueprintMapLibrary.Map_Find` (`local.Special Lookup`) `Floor Number`))
  (if (`KismetStringLibrary.IsNumeric` `Floor Number`)
    (if (< `Floor Number` (`local.Unknown`))
      (return (`KismetStringLibrary.Conv_StringToDouble` `Floor Number`))
      (else
        _))
    (elif _returnvalue
      (return _value)
      (else
        _)))
  (return (`local.Unknown`)))

(fn `Get Door Offset`
  (params (`Door Initial` :type "Vector Structure") (`Open Amount` :type "Float (double-precision)") (`Open Direction` :type "/Game/Caldoria/Blueprints/Enums/E_OpenDirection Enum" :default "NewEnumerator0"))
  (returns (`Door Destination` :type "Vector Structure"))
  (locals (Door :type "Transform Structure"))
  (switch `/Game/Caldoria/Blueprints/Enums/E_OpenDirection` `Open Direction`
    (:`NewEnumerator0`
      (return (`KismetMathLibrary.MakeVector` (- `Door Initial_X` `Open Amount`) `Door Initial_Y` `Door Initial_Z`)))
    (:`NewEnumerator1`
      (return (`KismetMathLibrary.MakeVector` (+ `Door Initial_X` `Open Amount`) `Door Initial_Y` `Door Initial_Z`)))))

(fn `GetIsLocked`
  (returns (IsLocked :type Boolean))
  (return (`self.DoorIsLocked`)))

(fn `GetIsOpen`
  (returns (`Door Is Open` :type Boolean))
  (bind _door_is_open (`/Game/Caldoria/Blueprints/BPI_Door.GetIsOpen` (`self.Instanced Elevator Doors`)))
  (return _door_is_open))

(fn `Setup Elevator Doors`
  (bind _asbp_elevator_doors (cast `/Game/Caldoria/Blueprints/BP_Elevator_Doors` (`ChildActorComponent.ChildActor` (`self.BP_Elevator_Doors`))))
  (set `self.Instanced Elevator Doors` _asbp_elevator_doors))

(fn `Setup Intercom`
  (`|ExecutionSequence`
    (:`then_0`
      (bind _asbp_elevator_hallway_intercom (cast `/Game/Caldoria/Blueprints/BP_Elevator_Hallway_Intercom` (`ChildActorComponent.ChildActor` (`self.BP_Elevator_Hallway_Intercom`))))
      (set `self.Instanced Elevator Intercom` _asbp_elevator_hallway_intercom))
    (:`then_1`
      (add `/Game/Caldoria/Blueprints/BP_Elevator_Hallway_Intercom.Call Button Pressed` (`self.Instanced Elevator Intercom`) (`|CreateDelegate` :!event `Request This Floor`)))))

(fn `Setup Speaker`
  (params (`Audio Source` :type "SoundBase Object Reference"))
  (`/Game/Caldoria/Blueprints/BP_Elevator_Hallway_Intercom.Set Speaker Audio` (`self.Instanced Elevator Intercom`) `Audio Source`))

(fn `UserConstructionScript`
  (`|ExecutionSequence`
    (:`then_0`)
    (:`then_1`
      ;[1 1 1] Set Door Number Sign
      (bind _returnvalue (`DecalComponent.CreateDynamicMaterialInstance` (`self.FloorNumberDecal`)))
      (bind _floor_index (`self.FloorIndexFromNumber` (`self.Floor Number`)))
      (`MaterialInstanceDynamic.SetScalarParameterValue` _returnvalue "Floor Number" _floor_index))))