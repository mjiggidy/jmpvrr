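; Elevator hallway intercom (old version) with a call button that fires CallButtonPressed when an Interact-tagged component overlaps its box.
; IlluminateButton and TurnOffLight fade the button glow in and out with timelines, guarded by lit and transitioning flags.
; Glow fade and pulsing are scalar parameters on a dynamic material instance created in the construction script.
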(event `self.Box.OnComponentBeginOverlap`
  (params (OverlappedComponent :type "PrimitiveComponent Object Reference") (OtherActor :type "Actor Object Reference") (OtherComp :type "PrimitiveComponent Object Reference") (OtherBodyIndex :type Integer) (bFromSweep :type Boolean) (SweepResult :type "HitResult Structure (by ref)"))
  (if (`ActorComponent.ComponentHasTag` OtherComp "Interact")
    (`self.Call Button Pressed`)))

(event `Illuminate Button`
  (params (Flashing :type Boolean))
  (`self.Set Is Flashing` Flashing)
  (if (`self.ButtonIsTransitioning`)
    _
    (elif (not (`self.IsLit`))
      (set `self.ButtonIsTransitioning` true)
      (bind (_direction _glow_amount) (`Timeline|Timeline` :!via `PlayFromStart`)
        (:`Update`
          (`self.Set Button Glow` _glow_amount))
        (:`Finished`
          (set `self.ButtonIsTransitioning` false)
          (set `self.IsLit` true))))))

(event `Turn Off Light`
  (if (`self.ButtonIsTransitioning`)
    _
    (elif (`self.IsLit`)
      (set `self.ButtonIsTransitioning` true)
      (`TimelineComponent.SetPlayRate` (`self.Timeline_0`) 2.0)
      (bind (_direction _glow_amount) (`Timeline|Timeline_0` :!via `PlayFromStart`)
        (:`Update`
          (`self.Set Button Glow` (- 1.0 _glow_amount))
          (`self.Set Is Flashing` false)
          (set `self.ButtonIsTransitioning` false)
          (set `self.IsLit` false))))))

(fn `Set Button Glow`
  (params (`Glow Amount` :type "Float (double-precision)"))
  (`MaterialInstanceDynamic.SetScalarParameterValue` (`self.Instanced Button Material`) "Glow Fade" `Glow Amount`))

(fn `Set Is Flashing`
  (params (`Is Flashing` :type Boolean))
  (`MaterialInstanceDynamic.SetScalarParameterValue` (`self.Instanced Button Material`) "Is Pulsing" (`KismetMathLibrary.Conv_BoolToDouble` `Is Flashing`)))

(fn `UserConstructionScript`
  (`|ExecutionSequence`
    (:`then_0`
      (bind _returnvalue (`PrimitiveComponent.CreateDynamicMaterialInstance` (`self.Cal_Elevator_Intercom_Button`) 0 null "None"))
      (set `self.Instanced Button Material` _returnvalue))))