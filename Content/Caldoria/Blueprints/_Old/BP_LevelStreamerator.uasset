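; Level streaming helper actor that loads or unloads several named sublevels on request.
; LoadMultpleLevels and UnloadMultipleLevels convert their Levels input to an array and pass it to recursive chained events that handle the first entry, remove it and call themselves.
; Stream calls are non-blocking; loading skips already loaded levels and makes new ones visible, with debug text printed for streamed levels.
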(event `LoadMultpleLevels`
  (params (Levels :type "Set of Name"))
  (bind _result (`BlueprintSetLibrary.Set_ToArray` Levels))
  (`self.LoadLevelChained` _result))

(event `LoadLevelChained`
  (params (`Temp Array` :type "Array of Name"))
  (bind _output (`|GetArrayItem` `Temp Array`))
  (if (`KismetArrayLibrary.Array_IsNotEmpty` `Temp Array`)
    (if (not (`LevelStreaming.IsLevelLoaded` (`GameplayStatics.GetStreamingLevel` _output)))
      (`GameplayStatics.LoadStreamLevel` _output true)
      ;[1 1 1] Debug
      (`KismetSystemLibrary.PrintText` (`|FormatText` "Stream In {level}" _output)))
    (`KismetArrayLibrary.Array_Remove` `Temp Array`)
    (`self.LoadLevelChained` `Temp Array`)))

(event `UnloadMultipleLevels`
  (params (Levels :type "Set of Name"))
  (bind _result (`BlueprintSetLibrary.Set_ToArray` Levels))
  (`self.UnloadLevelChained` _result))

(event `UnloadLevelChained`
  (params (`Temp Array` :type "Array of Name"))
  (bind _output (`|GetArrayItem` `Temp Array`))
  (if (`KismetArrayLibrary.Array_IsNotEmpty` `Temp Array`)
    (`GameplayStatics.UnloadStreamLevel` _output)
    (`KismetSystemLibrary.PrintText` (`|FormatText` "Stream Out {level}" _output))
    (`KismetArrayLibrary.Array_Remove` `Temp Array`)
    (`self.UnloadLevelChained` `Temp Array`)))

(fn `UserConstructionScript`)