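; Spring-loaded physical button that sinks when touched by components with the interactable tag, firing pressed and unpressed events, and resets when touch ends.
; CollisionBounds, sized from the mesh, records each toucher's entry position.
; Tick projects the first toucher's movement onto the right vector, slides the mesh along local Y up to the actuation distance, and triggers presses with a timeout.
; PushDirection only drives a construction-time debug arrow.
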(event `self.ReceiveBeginPlay`
  (set `self.Button Initial World Location` (`SceneComponent.K2_GetComponentLocation` (`self.Button Mesh`))))

(event `self.ReceiveTick`
  (params (DeltaSeconds :type "Float (single-precision)"))
  (bind _collision_bounds (`self.Collision Bounds`))
  (bind _returnvalue (`SceneComponent.GetRightVector` (`self.Collision Bounds`)))
  (if (`self.Button Being Touched`)
    (bind (_deelest_feela _initial_world_position) (`self.Get Deepest Interactable`))
    (bind _returnvalue_2 (`SceneComponent.K2_GetComponentLocation` _deelest_feela))
    (`KismetSystemLibrary.DrawDebugCoordinateSystem` (+ (`SceneComponent.K2_GetComponentLocation` _collision_bounds) (`KismetMathLibrary.InverseTransformLocation` (`SceneComponent.K2_GetComponentToWorld` _collision_bounds) (`KismetMathLibrary.ProjectVectorOnToVector` _returnvalue_2 _returnvalue))) (struct) 20.0 0.0 5.0)
    (bind _returnvalue_3 (`KismetMathLibrary.FClamp` (`KismetMathLibrary.Abs` (`KismetMathLibrary.VSize` (`KismetMathLibrary.ProjectVectorOnToVector` (- _returnvalue_2 _initial_world_position) _returnvalue))) 0.0 (`self.Actuation Distance (cm)`)))
    (`SceneComponent.K2_SetRelativeLocation` (`self.Button Mesh`) (`KismetMathLibrary.MakeVector` 0.0 (* _returnvalue_3 -1.0)) false false)
    (if (< _returnvalue_3 (`self.Actuation Distance (cm)`))
      (if (`self.Button Is Pressed`)
        (`self.Actuation Over`))
      (else
        (`self.Actuation Reached`)))))

(event `self.Collision Bounds.OnComponentBeginOverlap`
  (params (OverlappedComponent :type "PrimitiveComponent Object Reference") (OtherActor :type "Actor Object Reference") (OtherComp :type "PrimitiveComponent Object Reference") (OtherBodyIndex :type Integer) (bFromSweep :type Boolean) (SweepResult :type "HitResult Structure (by ref)"))
  (if (and (`KismetSystemLibrary.IsValid` OtherComp) (`ActorComponent.ComponentHasTag` OtherComp (`self.Interactable Tag`)))
    (`BlueprintMapLibrary.Map_Add` (`self.Currently Overlapping Components`) OtherComp (`SceneComponent.K2_GetComponentLocation` OtherComp))
    (if (not (`self.Button Being Touched`))
      (`self.ButtonTouchStart`))))

(event `self.Collision Bounds.OnComponentEndOverlap`
  (params (OverlappedComponent :type "PrimitiveComponent Object Reference") (OtherActor :type "Actor Object Reference") (OtherComp :type "PrimitiveComponent Object Reference") (OtherBodyIndex :type Integer))
  (if (`ActorComponent.ComponentHasTag` OtherComp (`self.Interactable Tag`))
    (bind _overlapping_interactables (`self.Get Interactable Components` (`PrimitiveComponent.GetOverlappingComponents` (`self.Collision Bounds`))))
    (if (not (`KismetMathLibrary.Conv_IntToBool` (`KismetArrayLibrary.Array_Length` _overlapping_interactables)))
      (`BlueprintMapLibrary.Map_Remove` (`self.Currently Overlapping Components`) OtherComp)
      (`self.ButtonTouchStop`))))

(event `Actuation Reached`
  (bind _returnvalue (`GameplayStatics.GetTimeSeconds`))
  (if (not (< (- _returnvalue (`self.Time Last Pressed`)) (`self.Timeout Duration (Seconds)`)))
    (set `self.Time Last Pressed` _returnvalue)
    (set `self.Button Is Pressed` true)
    (`self.ButtonPressed`)))

(event `Actuation Over`
  (set `self.Button Is Pressed` false)
  (`self.ButtonUnpressed`))

(event `Button Touch Begin`
  (set `self.Button Being Touched` true))

(event `Button Touch End`
  (set `self.Button Being Touched` false)
  (`SceneComponent.ResetRelativeTransform` (`self.Button Mesh`)))

(fn `Get Deepest Interactable`
  (returns (`Deelest Feela` :type "PrimitiveComponent Object Reference") (`Initial World Position` :type "Vector Structure"))
  (bind _currently_overlapping_components (`self.Currently Overlapping Components`))
  (bind _keys (`BlueprintMapLibrary.Map_Keys` _currently_overlapping_components))
  (bind _output (`|GetArrayItem` _keys))
  (return _output (`BlueprintMapLibrary.Map_Find` _currently_overlapping_components _output)))

(fn `Get Interactable Components`
  (params (Components :type "Array of PrimitiveComponent Object Reference"))
  (returns (`Overlapping Interactables` :type "Array of PrimitiveComponent Object Reference"))
  (locals (Interactables :type "Array of PrimitiveComponent Object Reference"))
  (bind _interactables (`local.Interactables`))
  (for _array_element Components
    (if (`ActorComponent.ComponentHasTag` _array_element (`self.Interactable Tag`))
      (`KismetArrayLibrary.Array_Add` _interactables _array_element)))
  (return _interactables))

(fn `GetFacingVector`
  (params (Direction :type "/Game/Caldoria/Blueprints/Enums/E_VectorDirections Enum" :default "NewEnumerator0") (Flip :type Boolean) (Component :type "SceneComponent Object Reference"))
  (returns (`Facing Vector` :type "Vector Structure"))
  (locals (Multiplier :type "Float (double-precision)" :default 1.0))
  (bind _multiplier (`local.Multiplier`))
  (if Flip
    (set `local.Multiplier` -1.0))
  (switch `/Game/Caldoria/Blueprints/Enums/E_VectorDirections` Direction
    (:`NewEnumerator0`
      (return (* (`SceneComponent.GetForwardVector` Component) _multiplier)))
    (:`NewEnumerator1`
      (return (* (`SceneComponent.GetRightVector` Component) _multiplier)))
    (:`NewEnumerator2`
      (return (* (`SceneComponent.GetUpVector` Component) _multiplier)))))

(fn `UserConstructionScript`
  (bind _collision_bounds (`self.Collision Bounds`))
  (bind _collision_bounds_2 (`self.Collision Bounds`))
  (bind _returnvalue (`SceneComponent.K2_GetComponentLocation` _collision_bounds_2))
  (bind (_origin _boxextent) (`KismetSystemLibrary.GetComponentBounds` (`self.Button Mesh`)))
  (bind _returnvalue_2 (+ _boxextent (`self.Bounds Padding`)))
  (`|ExecutionSequence`
    (:`then_0`
      ;[1 1 1] Static Mesh Setup
      (`StaticMeshComponent.SetStaticMesh` (`self.Button Mesh`) (`self.Button Static Mesh`)))
    (:`then_1`
      ;[1 1 1] Collision Setup
      (`KismetSystemLibrary.PrintString` (`KismetTextLibrary.Conv_TextToString` (`|FormatText` "Hey I saw {this}" (`KismetStringLibrary.Conv_VectorToString` _returnvalue_2))))
      (`SceneComponent.K2_SetWorldLocation` _collision_bounds (+ (`self.Bounds Position Offset`) _origin) false false)
      (`BoxComponent.SetBoxExtent` _collision_bounds _returnvalue_2 true))
    (:`then_2`
      ;[1 1 1] Bind Events
      (add `self.ButtonTouchStop` (`|CreateDelegate` :!event `Button Touch End`))
      (add `self.ButtonTouchStart` (`|CreateDelegate` :!event `Button Touch Begin`)))
    (:`then_3`
      (bind _facing_vector (`self.GetFacingVector` (`self.Push Direction`) (`self.Flip Push Direction`) _collision_bounds_2))
      (`KismetSystemLibrary.DrawDebugArrow` (+ (* _facing_vector 20.0) _returnvalue) _returnvalue 3.0 (struct :`G` 0.260379 :`B` 1.0 :`A` 1.0) 1.0 1.0))))