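; BPA_LevelStreamer is a helper that requests loading and unloading of streamed sublevels as areas change.
; It caches VRGameMode_JPVR on BeginPlay and forwards name sets to it as needed or not needed, leaving streaming to the game mode.
; Area swaps use set differences, so only sublevels unique to the new or old area are sent, loads first.
; Single-name functions wrap the name in a set and reuse the set-based events.
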(event `self.ReceiveBeginPlay`
  (bind _asvrgame_mode_jpvr (cast `/Game/_Player/VRGameMode_JPVR` (`GameplayStatics.GetGameMode`)))
  (set `self.GameMode` _asvrgame_mode_jpvr))

(event `Load Sublevels`
  (params (`Sublevel Names` :type "Set of Name"))
  (`/Game/_Player/VRGameMode_JPVR.SublevelsNeeded` (`self.GameMode`) `Sublevel Names`))

(event `Unload Sublevels`
  (params (`Sublevel Names` :type "Set of Name"))
  (`/Game/_Player/VRGameMode_JPVR.SublevelsNotNeeded` (`self.GameMode`) `Sublevel Names`))

(event `Load Sublevel Difference`
  (params (`New Area` :type "Set of Name (by ref)") (`Old Area` :type "Set of Name (by ref)"))
  (bind _result (`BlueprintSetLibrary.Set_Difference` `New Area` `Old Area`))
  (`/Game/_Player/VRGameMode_JPVR.SublevelsNeeded` (`self.GameMode`) _result))

(event `Unload Sublevel Difference`
  (params (`Current Area` :type "Set of Name (by ref)") (`Disposable Area` :type "Set of Name (by ref)"))
  (bind _result (`BlueprintSetLibrary.Set_Difference` `Disposable Area` `Current Area`))
  (`/Game/_Player/VRGameMode_JPVR.SublevelsNotNeeded` (`self.GameMode`) _result))

(event `Swap Sublevels`
  (params (`New Area` :type "Set of Name") (`Old Area` :type "Set of Name"))
  (`self.Load Sublevel Difference` `New Area` `Old Area`)
  (`self.Unload Sublevel Difference` `New Area` `Old Area`))

(fn `Load Sublevel`
  (params (`Sublevel Name` :type Name))
  (locals (NameAsSet :type "Set of Name"))
  (bind _nameasset (`local.NameAsSet`))
  (`BlueprintSetLibrary.Set_Add` _nameasset `Sublevel Name`)
  (`self.Load Sublevels` _nameasset))

(fn `Unload Sublevel`
  (params (`Sublevel Name` :type Name))
  (locals (NameAsSet :type "Set of Name"))
  (bind _nameasset (`local.NameAsSet`))
  (`BlueprintSetLibrary.Set_Add` _nameasset `Sublevel Name`)
  (`self.Unload Sublevels` _nameasset))