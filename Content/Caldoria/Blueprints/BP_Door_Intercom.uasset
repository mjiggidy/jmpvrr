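; BP_Door_Intercom is a door intercom that plays a settable audio message and lights its button glow.
; BeginPlay configures a child BP_SpringLoadedButton, creates its dynamic material and binds button-press and audio play-state events.
; Glow fades in or out through timelines at randomized rates, and Tick adds the audio's cooked envelope amplitude so it pulses during playback.
; PropagateMessage re-broadcasts presses through CallButtonPressed.
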(event `self.ReceiveBeginPlay`
  (`self.Setup Button`)
  (`self.Setup Audio`))

(event `self.ReceiveTick`
  (params (DeltaSeconds :type "Float (single-precision)"))
  (if (`AudioComponent.IsPlaying` (`self.Audio`))
    (bind _amplitude (`self.Get Scaled Amplitude` 20.0))
    (`self.Set Glow Intensity` (+ _amplitude (`self.Current Glow Intensity`)))))

(event `Play Message`
  (if (not (`AudioComponent.IsPlaying` (`self.Audio`)))
    (`AudioComponent.Play` (`self.Audio`) 0.0)))

(event `Activate Light`
  (`TimelineComponent.SetPlayRate` (`self.Fade In Curve`) (`KismetMathLibrary.RandomFloatInRange` 2.0 4.0))
  (bind _returnvalue (`MaterialInstanceDynamic.K2_GetScalarParameterValue` (`self.Button Material`) (`self.Glow Property Name`)))
  (bind _output_get (set `self.Old Glow Intensity` _returnvalue))
  (bind (_direction _fade) (`Timeline|Fade In Curve` :!via `PlayFromStart`)
    (:`Update`
      (bind _returnvalue_2 (`KismetMathLibrary.Lerp` _output_get (`self.Max Glow Intensity`) _fade))
      (`self.Set Glow Intensity` _returnvalue_2)
      (set `self.Current Glow Intensity` _returnvalue_2))))

(event `Deactivate Light`
  (`TimelineComponent.SetPlayRate` (`self.Fade Out Curve`) (`KismetMathLibrary.RandomFloatInRange` 2.0 4.0))
  (bind _returnvalue (`MaterialInstanceDynamic.K2_GetScalarParameterValue` (`self.Button Material`) (`self.Glow Property Name`)))
  (bind _output_get (set `self.Old Glow Intensity` _returnvalue))
  (bind (_direction _fade) (`Timeline|Fade Out Curve` :!via `PlayFromStart`)
    (:`Update`
      (bind _returnvalue_2 (`KismetMathLibrary.Lerp` _output_get 0.0 _fade))
      (`self.Set Glow Intensity` _returnvalue_2)
      (set `self.Current Glow Intensity` _returnvalue_2))))

(event `Propagate Message`
  (`self.ButtonPressed`))

(fn `Get Scaled Amplitude`
  (params (Scale :type "Float (double-precision)" :default 20.0))
  (returns (Amplitude :type "Float (double-precision)"))
  (bind (_outenvelopedata _returnvalue) (`AudioComponent.GetCookedEnvelopeData` (`self.Audio`)))
  (if _returnvalue
    (return (* Scale _outenvelopedata))
    (else
      (return 0.0))))

(fn `Set Glow Intensity`
  (params (Intensity :type "Float (double-precision)"))
  (`MaterialInstanceDynamic.SetScalarParameterValue` (`self.Button Material`) (`self.Glow Property Name`) Intensity))

(fn `Set Message`
  (params (`New Message` :type "SoundWave Soft Object Reference"))
  (`AudioComponent.SetSound` (`self.Audio`) (`|ConvertAsset` `New Message`)))

(fn `Setup Audio`
  (add `AudioComponent.OnAudioPlayStateChanged` (`self.Audio`) (`|CreateDelegate` :!event `ToggleButtonGlow`)))

(fn `Setup Button`
  (bind _instanced_spring_loaded_button (`self.Instanced Spring Loaded Button`))
  (`|ExecutionSequence`
    (:`then_0`
      (bind _asbp_spring_loaded_button (cast `/Game/Caldoria/Blueprints/BP_SpringLoadedButton` (`ChildActorComponent.ChildActor` (`self.BP_SpringLoadedButton`))))
      (set `self.Instanced Spring Loaded Button` _asbp_spring_loaded_button))
    (:`then_1`
      (bind _button_component (`/Game/Caldoria/Blueprints/BP_SpringLoadedButton.Get Button Component` _instanced_spring_loaded_button))
      (bind _returnvalue (`PrimitiveComponent.CreateDynamicMaterialInstance` _button_component 0 null "None")) ; Test This
      (set `self.Button Material` _returnvalue))
    (:`then_2`
      (set `/Game/Caldoria/Blueprints/BP_SpringLoadedButton.Timeout Duration (Seconds)` (`self.Button Timeout`) _instanced_spring_loaded_button))
    (:`then_3`
      (add `/Game/Caldoria/Blueprints/BP_SpringLoadedButton.ButtonPressed` _instanced_spring_loaded_button (`|CreateDelegate` :!event `Propagate Message`)))))

(fn `ToggleButtonGlow`
  (params (PlayState :type "EAudioComponentPlayState Enum" :default "Playing"))
  (switch `EAudioComponentPlayState` PlayState
    (:`Playing`
      (`self.Activate Light`))
    (:`Stopped`
      (`self.Deactivate Light`))))

(fn `UserConstructionScript`
  (`|ExecutionSequence`))