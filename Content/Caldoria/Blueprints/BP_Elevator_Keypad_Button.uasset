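; Physical elevator keypad button in Caldoria that either queues a floor or toggles the door, depending on its mode.
; An "Interact"-tagged component entering the box calls the floor or door request dispatcher, and each tick the button mesh's offset follows that component, clamped to a short travel.
; A dynamic material instance created at construction picks the key symbol from an atlas and drives glow and blinking.
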(event `self.ReceiveTick`
  (params (DeltaSeconds :type "Float (single-precision)"))
  (bind _overlapper (`self.Overlapper`))
  (bind _returnvalue (`SceneComponent.K2_GetComponentLocation` _overlapper))
  (bind (_returnvalue_x _returnvalue_y) (`KismetMathLibrary.BreakVector` (- (`PrimitiveComponent.GetClosestPointOnCollision` (`self.Box`) _returnvalue "None") _returnvalue)))
  (if (`KismetSystemLibrary.IsValid` _overlapper)
    (`SceneComponent.K2_SetRelativeLocation` (`self.Cal_Elevator_Panel_Button`) (`KismetMathLibrary.MakeVector` (`KismetMathLibrary.FClamp` (+ _returnvalue_y 2.45) 0.0 0.5)) false false)
    (`KismetSystemLibrary.PrintText` (`|FormatText` "Button relative location: {location}" (`KismetStringLibrary.Conv_VectorToString` (`SceneComponent.RelativeLocation` (`self.Cal_Elevator_Panel_Button`)))))))

(event `ButtonPressed`
  (switch `/Game/Caldoria/Blueprints/E_Elevator_Keypad_Button_Modes` (`self.Mode`)
    (:`NewEnumerator0`
      (`self.FloorRequested` (`self.Floor`)))
    (:`NewEnumerator1`
      (`self.Door Requested`))))

(event `self.Box.OnComponentBeginOverlap`
  (params (OverlappedComponent :type "PrimitiveComponent Object Reference") (OtherActor :type "Actor Object Reference") (OtherComp :type "PrimitiveComponent Object Reference") (OtherBodyIndex :type Integer) (bFromSweep :type Boolean) (SweepResult :type "HitResult Structure (by ref)"))
  (if (`ActorComponent.ComponentHasTag` OtherComp "Interact")
    (set `self.Overlapper` OtherComp)
    (`self.ButtonPressed`)))

(event `self.Box.OnComponentEndOverlap`
  (params (OverlappedComponent :type "PrimitiveComponent Object Reference") (OtherActor :type "Actor Object Reference") (OtherComp :type "PrimitiveComponent Object Reference") (OtherBodyIndex :type Integer))
  (if (`ActorComponent.ComponentHasTag` OtherComp "Interact")
    (set `self.Overlapper` null)
    (`SceneComponent.K2_SetRelativeLocation` (`self.Cal_Elevator_Panel_Button`) (0.0 0.0 0.0) false false)
    (`KismetSystemLibrary.PrintText` (`|FormatText` "Button back to: {location}" (`KismetStringLibrary.Conv_VectorToString` (`SceneComponent.RelativeLocation` (`self.Cal_Elevator_Panel_Button`)))))))

(fn `Set Glow Intensity`
  (params (Intensity :type "Float (double-precision)"))
  (`MaterialInstanceDynamic.SetScalarParameterValue` (`self.Instanced Material`) "Glow Fade" Intensity))

(fn `SetMode`
  (params (Mode :type "/Game/Caldoria/Blueprints/E_Elevator_Keypad_Button_Modes Enum" :default "NewEnumerator0") (Floor :type "/Game/Caldoria/Blueprints/BP_Elevator_Hallway Object Reference"))
  (bind _output_get (set `self.Mode` Mode))
  (switch `/Game/Caldoria/Blueprints/E_Elevator_Keypad_Button_Modes` _output_get
    (:`NewEnumerator0`
      (set `self.Floor` Floor))))

(fn `SetupButton`
  (params (Mode :type "/Game/Caldoria/Blueprints/E_Elevator_Keypad_Button_Modes Enum" :default "NewEnumerator0") (Floor :type "/Game/Caldoria/Blueprints/BP_Elevator_Hallway Object Reference"))
  (set `self.Mode` Mode)
  (set `self.Floor` Floor)
  (`self.UpdateKeySymbol`))

(fn `TurnButtonOff`
  (bind _instanced_material (`self.Instanced Material`))
  (`MaterialInstanceDynamic.SetScalarParameterValue` _instanced_material "Glow Fade" 0.0)
  (`MaterialInstanceDynamic.SetScalarParameterValue` _instanced_material "Is Blinking" 0.0))

(fn `TurnButtonOn`
  (params (Blinking :type Boolean))
  (bind _instanced_material (`self.Instanced Material`))
  (`MaterialInstanceDynamic.SetScalarParameterValue` _instanced_material "Glow Fade" 1.0)
  (`MaterialInstanceDynamic.SetScalarParameterValue` _instanced_material "Is Blinking" (`KismetMathLibrary.Conv_BoolToDouble` Blinking)))

(fn `UpdateKeySymbol`
  (locals (AtlasIndex :type Integer))
  (bind _floor_number (`/Game/Caldoria/Blueprints/BP_Elevator_Hallway.Floor Number` (`self.Floor`)))
  (switch `/Game/Caldoria/Blueprints/E_Elevator_Keypad_Button_Modes` (`self.Mode`)
    (:`NewEnumerator0`
      (if (`KismetStringLibrary.IsNumeric` _floor_number)
        (set `local.AtlasIndex` (`KismetStringLibrary.Conv_StringToInt` _floor_number))
        (else
          (set `local.AtlasIndex` 5))))
    (:`NewEnumerator1`
      (set `local.AtlasIndex` 6)))
  (`MaterialInstanceDynamic.SetScalarParameterValue` (`self.Instanced Material`) "Floor Number" (`KismetMathLibrary.Conv_IntToDouble` (`local.AtlasIndex`))))

(fn `UserConstructionScript`
  (bind _floor (`self.Floor`))
  (bind _returnvalue (`PrimitiveComponent.CreateDynamicMaterialInstance` (`self.Cal_Elevator_Panel_Button`) 0 "/Game/Caldoria/Materials/_TEMP/M_ElevatorKeypadButton.M_ElevatorKeypadButton" "None"))
  (set `self.Instanced Material` _returnvalue)
  (`self.SetupButton` (`self.Mode`) (`self.Floor`))
  (bind _output_get (set `self.Initial Location` (`SceneComponent.RelativeLocation` (`self.Cal_Elevator_Panel_Button`))))
  (if (`KismetSystemLibrary.IsValid` _floor)
    (bind _returnvalue_2 (`KismetStringLibrary.BuildString_Vector` "" "" _output_get))
    (`KismetSystemLibrary.PrintText` (`|FormatText` "Button {name} at {position}" (`/Game/Caldoria/Blueprints/BP_Elevator_Hallway.Floor Number` _floor) _returnvalue_2))
    (else
      (`KismetSystemLibrary.PrintText` (`|FormatText` "Button <-> at {position}" _returnvalue_2)))))